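; Tutorial vent cap (likely, per the TuT name) that ages and falls loose when the time gun is used on it, once activated.
; Activate arms it, then OnTimeGun plays a timeline driving the dynamic material's Age parameter.
; When the timeline finishes, the cap mesh starts simulating physics.
; The construction script creates the material instance; an extra popping impulse is left disconnected.
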(event Custom|Activate
  (Variables|Default|SetActivated? true))

(event EventBeginPlay)

(event Collision|EventActorBeginOverlap
  (params (OtherActor :type Actor%20Object%20Reference)))

(event EventTick
  (params (DeltaSeconds :type Float%20%28single-precision%29)))

(event EventOnTimeGun
  (params (Location :type Vector :default "0, 0, 0"))
  (if (Variables|Default|GetActivated?)
    ;[1 1 1] Aging + Falling down
    (bind _aging (Timeline|Timeline_0 Play)
      (:Update
        (Rendering|Material|SetScalarParameterValue (Variables|Default|GetMaterial) "Age" _aging :!class /Script/Engine.MaterialInstanceDynamic))
      (:Finished
        (Physics|SetSimulatePhysics (Variables|Default|GetSM_VentCapOpen) true)))))

(fn ConstructionScript
  (bind _returnvalue (Rendering|Material|CreateDynamicMaterialInstance 0 "/Game/Architecture/Source/VentCapOpen/M_VentCapOpen_Inst.M_VentCapOpen_Inst" :!class /Script/Engine.PrimitiveComponent))
  (bind _output_get (Variables|Default|SetMaterial _returnvalue))
  (Rendering|Material|SetMaterial 0 _output_get)
  (Rendering|Material|SetScalarParameterValue (Variables|Default|GetMaterial) "None" 0.0 :!class /Script/Engine.MaterialInstanceDynamic))