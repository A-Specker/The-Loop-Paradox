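; Lift actor with sliding double doors and a continuously flickering light.
; CloseDoors runs only once, enabling the BoxNoOut collision and sliding both doors via a timeline with mirrored offsets.
; OpenDoors disables that collision and plays a separate timeline on the same doors.
; Tick restarts a flicker timeline whenever it finishes, driving the point light intensity and the emissive strength of a dynamic material created in construction.
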(event Custom|CloseDoors
  (if (not (Variables|Default|Getclose))
    (Variables|Default|Setclose true)
    (Collision|SetCollisionEnabled (Variables|Default|GetBox_No_Out) "QueryAndPhysics")
    (bind _doorclose (Timeline|CloseLiftLeft Play)
      (:Update
        (Transformation|SetRelativeLocation (Variables|Default|GetDoorLeft) (Math|Vector|MakeVector -12.0 _doorclose 0.0) false)
        (Transformation|SetRelativeLocation (Variables|Default|GetDoorRight) (Math|Vector|MakeVector -12.0 (* _doorclose -1.0) 0.0) false)))))

(event Custom|OpenDoors
  (Collision|SetCollisionEnabled (Variables|Default|GetBox_No_Out) "NoCollision")
  (bind _openfunction (Timeline|OpenDoorsTimeline Play)
    (:Update
      (Transformation|SetRelativeLocation (Variables|Default|GetDoorLeft) (Math|Vector|MakeVector -12.0 _openfunction 0.0) false)
      (Transformation|SetRelativeLocation (Variables|Default|GetDoorRight) (Math|Vector|MakeVector -12.0 (* _openfunction -1.0) 0.0) false))))

(event EventTick
  (params (DeltaSeconds :type Float%20%28single-precision%29))
  (if (not (Variables|Default|GetIsFlickering))
    (Variables|Default|SetIsFlickering true)
    (bind _flicker (Timeline|Flickering PlayFromStart)
      (:Update
        (Rendering|Material|SetScalarParameterValue (Variables|Default|GetLiftLight) "EmmisiveStrength" (* _flicker 1e+01) :!class /Script/Engine.MaterialInstanceDynamic)
        (Rendering|Components|Light|SetIntensity (Variables|Default|GetPointLight) (* (* _flicker 1e+01) 1e+03)))
      (:Finished
        (Variables|Default|SetIsFlickering false)))))

(event EventBeginPlay
  (Collision|SetCollisionEnabled (Variables|Default|GetBox_No_Out) "NoCollision"))

(fn ConstructionScript
  (bind _returnvalue (Rendering|Material|CreateDynamicMaterialInstance "/Game/Architecture/Source/Lift/M_Lift.M_Lift" :!class /Script/Engine.KismetMaterialLibrary))
  (bind _output_get (Variables|Default|SetLiftLight _returnvalue))
  (Rendering|Material|SetMaterial (Variables|Default|GetSM_Lift) 0 _output_get))