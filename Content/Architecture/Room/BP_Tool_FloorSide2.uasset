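; Room-building tool Blueprint that lays out a straight floor-side strip from repeated mesh instances.
; The construction script keeps Size.X, forces a fixed depth and zero height, then fills an instanced static mesh component along local X, one instance per whole 200-unit step.
; GetSize reports Size in 200-unit tiles with Z fixed at one.
; The event graph holds no runtime logic.
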(event EventBeginPlay)

(event Collision|EventActorBeginOverlap
  (params (OtherActor :type Actor%20Object%20Reference)))

(event EventTick
  (params (DeltaSeconds :type Float%20%28single-precision%29)))

(fn ConstructionScript
  (bind _returnvalue (AddComponent|AddInstancedStaticMeshComponent false))
  (Variables|Default|SetFloorElement _returnvalue)
  ;[1 1 1] Only X and Y scaling allowed
  (bind _output_get (Variables|Default|SetSize (Math|Vector|MakeVector (.X (Math|Vector|BreakVector (Variables|Default|GetSize))) 5e+01 0.0)))
  ;[1 1 1] For X and Y
  (for _index (range 1 (.ReturnValue (Math|Float|Division(WholeandRemainder) (.X (Math|Vector|BreakVector _output_get)) 2e+02)))
    ;[1 1 1] Add Instances
    (Components|InstancedStaticMesh|AddInstance (Variables|Default|GetFloorElement) (Math|Transform|MakeTransform (Math|Vector|MakeVector (* _index 2e+02) 0.0 0.0)))))

(fn GetSize
  (bind _size (Variables|Default|GetSize))
  (bind _returnvalue (/ _size 2e+02))
  (return (Math|Vector|MakeVector (.x _returnvalue) (.y _returnvalue) 1.0)))