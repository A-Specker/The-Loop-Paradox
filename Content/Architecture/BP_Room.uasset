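; BP_Room is a procedural room actor that builds a floor plane and perimeter walls from a 2D Size value in the construction script.
; It flattens Size to X and Y, scales the plane to match and sets tiling on a dynamic material instance so the texture follows the size.
; Wall segments are placed at fixed intervals along all four edges as instances of one instanced static mesh component.
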(event EventBeginPlay)

(event Collision|EventActorBeginOverlap
  (params (OtherActor :type Actor%20Object%20Reference)))

(event EventTick
  (params (DeltaSeconds :type Float%20%28single-precision%29)))

(fn ConstructionScript
  ;[1 1 1] Only X and Y scaling allowed
  (Variables|Default|SetSize (Math|Vector|MakeVector (.X (Math|Vector|BreakVector (Variables|Default|GetSize))) (.Y (Math|Vector|BreakVector (Variables|Default|GetSize))) 0.0))
  ;[1 1 1] Correct Scaling
  (Transformation|SetRelativeScale3D (Variables|Default|GetPlane) (CallFunction|GetSize))
  ;[1 1 1] Texture Tiling
  (bind _returnvalue (Rendering|Material|CreateDynamicMaterialInstance (Variables|Default|GetMaterial) :!class /Script/Engine.KismetMaterialLibrary))
  (Rendering|Material|SetScalarParameterValue _returnvalue "TilingX" (.Y (Math|Vector|BreakVector (/ (Variables|Default|GetSize) 2e+02))) :!class /Script/Engine.MaterialInstanceDynamic)
  (Rendering|Material|SetScalarParameterValue _returnvalue "TilingY" (.X (Math|Vector|BreakVector (/ (Variables|Default|GetSize) 2e+02))) :!class /Script/Engine.MaterialInstanceDynamic)
  (Rendering|Material|SetMaterial (Variables|Default|GetPlane) 0 _returnvalue)
  (CallFunction|InitializeMeshes)
  (for _index (range 0 (.ReturnValue (Math|Float|Division(WholeandRemainder) (.X (Math|Vector|BreakVector (Variables|Default|GetSize))) 4e+02)))
    (CallFunction|AddWallXLeft _index)
    (CallFunction|AddWallXRight _index))
  (for _index_2 (range 0 (.ReturnValue (Math|Float|Division(WholeandRemainder) (.Y (Math|Vector|BreakVector (Variables|Default|GetSize))) 4e+02)))
    (CallFunction|AddWallYDown _index_2)
    (CallFunction|AddWallYUp _index_2)))

(fn GetSize
  (bind _size (Variables|Default|GetSize))
  (bind _returnvalue (/ _size 2e+02))
  (return (Math|Vector|MakeVector (.x _returnvalue) (.y _returnvalue) 1.0)))

(fn InitializeMeshes
  (bind _returnvalue (AddComponent|AddInstancedStaticMeshComponent false))
  (Variables|Default|SetWallStandard _returnvalue))

(fn AddWallXLeft
  (params (Index :type Integer))
  (Components|InstancedStaticMesh|AddInstance (Variables|Default|GetWallStandard) (Math|Transform|MakeTransform (Math|Vector|MakeVector (* Index 4e+02) 0.0 0.0) "90.000000,-90.000000, 0" "2.000000,2.000000,2.000000")))

(fn AddWallYDown
  (params (Index :type Integer))
  (Components|InstancedStaticMesh|AddInstance (Variables|Default|GetWallStandard) (Math|Transform|MakeTransform (Math|Vector|MakeVector 0.0 (* Index 4e+02) 0.0) "90.000000,0.000000, 0" "2.000000,2.000000,2.000000")))

(fn AddWallXRight
  (params (Index :type Integer))
  (Components|InstancedStaticMesh|AddInstance (Variables|Default|GetWallStandard) (Math|Transform|MakeTransform (Math|Vector|MakeVector (* Index 4e+02) (.Y (Math|Vector|BreakVector (Variables|Default|GetSize))) 0.0) "90.000000,-90.000000, 0" "2.000000,2.000000,2.000000")))

(fn AddWallYUp
  (params (Index :type Integer))
  (Components|InstancedStaticMesh|AddInstance (Variables|Default|GetWallStandard) (Math|Transform|MakeTransform (Math|Vector|MakeVector (.X (Math|Vector|BreakVector (Variables|Default|GetSize))) (* Index 4e+02) 0.0) "90.000000,0.000000, 0" "2.000000,2.000000,2.000000")))