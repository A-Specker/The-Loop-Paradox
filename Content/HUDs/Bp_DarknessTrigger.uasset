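; Trigger actor that drives a post-process effect, apparently darkness, based on how close the player is to its center.
; Overlap events flag when the player is inside, and Tick then sets the PostProcess blend weight to one minus the distance.
; GetDistance computes the player capsule's distance to the Cube component, normalized by the Sphere's scaled radius.
; Leaving clears the flag and deactivates the PostProcess component.
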(event Collision|EventActorBeginOverlap
  (params (OtherActor :type Actor%20Object%20Reference))
  (if (== OtherActor (Game|GetPlayerCharacter 0))
    (Variables|Default|SetisTriggered true)))

(event Collision|EventActorEndOverlap
  (params (OtherActor :type Actor%20Object%20Reference))
  (if (== OtherActor (Game|GetPlayerCharacter 0))
    (Variables|Default|SetisTriggered false)
    (Components|Activation|Deactivate (Variables|Default|GetPostProcess))))

(event EventTick
  (params (DeltaSeconds :type Float%20%28single-precision%29))
  (if (Variables|Default|GetisTriggered)
    (bind _distance (CallFunction|GetDistance))
    (bind _output_get (Variables|Default|SetDistance _distance))
    (Variables|/Script/Engine.PostProcessComponent|SetBlendWeight (Variables|Default|GetPostProcess) (- 1.0 _output_get))))

(fn ConstructionScript)

(fn GetDistance
  (bind _returnvalue (Game|GetPlayerCharacter 0))
  (bind _cube (Variables|Default|GetCube))
  (bind _returnvalue_2 (Transformation|GetWorldLocation _cube))
  (bind _capsulecomponent (Variables|/Script/Engine.Character|GetCapsuleComponent _returnvalue))
  (bind _returnvalue_3 (Transformation|GetWorldLocation _capsulecomponent))
  (bind _returnvalue_4 (- _returnvalue_3 _returnvalue_2))
  (bind (_x _y _z) (Math|Vector|BreakVector _returnvalue_4))
  (return (/ (Math|Float|Sqrt (+ (Math|Float|Power (Math|Float|Absolute(Float) _x) 2.0) (Math|Float|Power (Math|Float|Absolute(Float) _y) 2.0) (Math|Float|Power (Math|Float|Absolute(Float) _z) 2.0))) (Components|Sphere|GetScaledSphereRadius (Variables|Default|GetSphere)))))