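; Ventilator actor that the time gun toggles on and off, pushing the player with wind while on.
; Toggling switches the child fan actor and notifies pickables in the Box, which are also notified on entering or leaving while on.
; Tick applies force along the Arrow while the player overlaps the actor.
; The construction script counter-scales the fan against root scale.
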(event OnComponentBeginOverlap(Box)
  (params (OtherActor :type Actor%20Object%20Reference) (OtherComp :type Primitive%20Component%20Object%20Reference) (OtherBodyIndex :type Integer) (bFromSweep :type Boolean) (SweepResult :type Hit%20Result%20Structure%20%28by%20ref%29))
  (if (Variables|Default|GetOn?)
    (Class|VentilatorInterface|OnVentilator(Message) (Utilities|Array|Get(acopy) (Actor|GetComponentsByClass OtherActor "/Game/Blueprints/BP_Pickable.BP_Pickable_C")))))

(event OnComponentEndOverlap(Box)
  (params (OtherActor :type Actor%20Object%20Reference) (OtherComp :type Primitive%20Component%20Object%20Reference) (OtherBodyIndex :type Integer))
  (if (Variables|Default|GetOn?)
    (Class|VentilatorInterface|OnVentilator(Message) (Utilities|Array|Get(acopy) (Actor|GetComponentsByClass OtherActor "/Game/Blueprints/BP_Pickable.BP_Pickable_C")))))

(event Collision|EventActorBeginOverlap
  (params (OtherActor :type Actor%20Object%20Reference))
  (if (== OtherActor (Game|GetPlayerCharacter 0))
    (Variables|Default|SetInsideVentilator true)))

(event EventTick
  (params (DeltaSeconds :type Float%20%28single-precision%29))
  (if (Variables|Default|GetOn?)
    (if (Variables|Default|GetInsideVentilator)
      (Physics|AddForce (Variables|/Script/Engine.Character|GetCharacterMovement (Game|GetPlayerCharacter 0)) (* (Math|Vector|Normalize (Math|Vector|GetForwardVector (Variables|Default|GetArrow))) (Variables|Default|GetStrength))))))

(event Collision|EventActorEndOverlap
  (params (OtherActor :type Actor%20Object%20Reference))
  (if (== OtherActor (Game|GetPlayerCharacter 0))
    (Variables|Default|SetInsideVentilator false)))

(event EventOnTimeGun
  (params (Location :type Vector :default "0, 0, 0"))
  (bind _box (Variables|Default|GetBox))
  (bind _overlappingactors (Collision|GetOverlappingActors _box 0 :!class /Script/Engine.PrimitiveComponent))
  (if (Variables|Default|GetOn?)
    (Variables|Default|SetOn? false)
    (else
      (Variables|Default|SetOn? true)))
  (bind _asbp_fanrotate (Utilities|Casting|CastToBP_Fanrotate (Variables|/Script/Engine.ChildActorComponent|GetChildActor (Variables|Default|GetBP_Fanrotate))))
  (Default|Switch _asbp_fanrotate)
  (if (!= (Utilities|Array|Length _overlappingactors) 0)
    (for _array_element _overlappingactors
      (Class|VentilatorInterface|OnVentilator(Message) (Utilities|Array|Get(acopy) (Actor|GetComponentsByClass _array_element "/Game/Blueprints/BP_Pickable.BP_Pickable_C"))))))

(fn ConstructionScript
  (bind _defaultsceneroot (Variables|Default|GetDefaultSceneRoot))
  (bind _returnvalue (Transformation|GetWorldScale _defaultsceneroot))
  (bind (_x _y _z) (Math|Vector|BreakVector _returnvalue))
  (Transformation|SetRelativeScale3D (Variables|Default|GetBP_Fanrotate) (Math|Vector|MakeVector (/ 1.0 _x) (/ 1.0 _y) (/ 1.0 _z))))