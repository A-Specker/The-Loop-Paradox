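; Hanging lamp actor that switches its point light and glowing material on and off.
; The construction script creates a dynamic M_Hanglamp material instance, applies it to the lamp mesh and starts it with zero emissive.
; Each Trigger event flips a Triggered flag, setting light intensity and emissive strength to either their configured values or zero.
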(event Custom|Trigger
  (if (Variables|Default|GetTriggered)
    (Variables|Default|SetTriggered false)
    (Rendering|Components|Light|SetIntensity (Variables|Default|GetPointLight) 0.0)
    (Rendering|Material|SetScalarParameterValue (Variables|Default|GetMaterial) "Emissive" 0.0 :!class /Script/Engine.MaterialInstanceDynamic)
    (else
      (Variables|Default|SetTriggered true)
      (Rendering|Components|Light|SetIntensity (Variables|Default|GetPointLight) (Variables|Default|GetLightIntensity))
      (Rendering|Material|SetScalarParameterValue (Variables|Default|GetMaterial) "Emissive" (Variables|Default|GetMatIntensity) :!class /Script/Engine.MaterialInstanceDynamic))))

(event EventBeginPlay)

(event Collision|EventActorBeginOverlap
  (params (OtherActor :type Actor%20Object%20Reference)))

(event EventTick
  (params (DeltaSeconds :type Float%20%28single-precision%29)))

(fn ConstructionScript
  (bind _returnvalue (Rendering|Material|CreateDynamicMaterialInstance "/Game/Architecture/Room/Source/HangLamp/M_Hanglamp.M_Hanglamp" :!class /Script/Engine.KismetMaterialLibrary))
  (bind _output_get (Variables|Default|SetMaterial _returnvalue))
  (Rendering|Material|SetScalarParameterValue _output_get "Emissive" 0.0 :!class /Script/Engine.MaterialInstanceDynamic)
  (Rendering|Material|SetMaterial (Variables|Default|GetSM_HangLamp) 0 _output_get))