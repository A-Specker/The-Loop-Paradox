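; BP_GeneratorStatic is a generator prop whose On flag decides whether it appears running or switched off.
; The construction script gives the body a dynamic M_Generator material and sets its emissive parameter from that flag.
; When on, BeginPlay attaches a looping-or-one-shot Generator_Cue sound to the body at reduced volume, and Tick rotates the element mesh by RotationSpeed each frame, without delta-time scaling.
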(event EventBeginPlay
  (if (Variables|Default|GetOn?)
    (bind _returnvalue (Class|GameplayStatics|PlaySoundAttached "/Game/Audio/Generator/Generator_Cue.Generator_Cue" (Variables|Default|GetSM_GeneratorBody)))
    (bind _output_get (Variables|Default|SetSound _returnvalue))
    (Audio|Components|Audio|SetVolumeMultiplier _output_get 0.4 :!class /Script/Engine.AudioComponent)))

(event Collision|EventActorBeginOverlap
  (params (OtherActor :type Actor%20Object%20Reference)))

(event EventTick
  (params (DeltaSeconds :type Float%20%28single-precision%29))
  (if (Variables|Default|GetOn?)
    (Transformation|AddLocalRotation (Variables|Default|GetSM_GeneratorElem) (Class|KismetMathLibrary|MakeRot 0.0 (Variables|Default|GetRotationSpeed) 0.0) false)))

(fn ConstructionScript
  (bind _returnvalue (Rendering|Material|CreateDynamicMaterialInstance "/Game/General/Sources/Generator/M_Generator.M_Generator" :!class /Script/Engine.KismetMaterialLibrary))
  (bind _output_get (Variables|Default|SetMaterial _returnvalue))
  (Rendering|Material|SetMaterial (Variables|Default|GetSM_GeneratorBody) 0 _output_get)
  (if (Variables|Default|GetOn?)
    (Rendering|Material|SetScalarParameterValue (Variables|Default|GetMaterial) "Emmisive" 6.0 :!class /Script/Engine.MaterialInstanceDynamic)
    (else
      (Rendering|Material|SetScalarParameterValue (Variables|Default|GetMaterial) "Emmisive" 0.0 :!class /Script/Engine.MaterialInstanceDynamic))))