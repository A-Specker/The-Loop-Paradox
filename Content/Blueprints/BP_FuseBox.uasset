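; Interactable fuse box that takes the player's fuse and starts a timed escape window until the fuse breaks.
; On interact with a fuse held, it hides and resets the physics fuse mesh, triggers its BP_FuseStandard child, updates character prompts and countdown, and fires CallStartCountdown.
; A timer using the character's TimeFuseBreak runs FuseBreak, which buzzes, retriggers the child, drops the visible fuse with physics and removes escape.
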(event Custom|Fuse%20Break
  (bind _sm_fuse (Variables|Default|GetSM_Fuse))
  (Class|GameplayStatics|PlaySoundAttached "/Game/Audio/Sounds/ElectricBuzz_Cue.ElectricBuzz_Cue" (Variables|Default|GetStaticMesh))
  (bind _asbp_fuse_standard (Utilities|Casting|CastToBP_FuseStandard (Variables|/Script/Engine.ChildActorComponent|GetChildActor (Variables|Default|GetBP_FuseStandard))))
  (Default|Trigger _asbp_fuse_standard)
  (Rendering|SetVisibility _sm_fuse true false)
  (Physics|SetSimulatePhysics _sm_fuse true)
  (Default|RemoveEscape (.AsThird%20Person%20Character (Utilities|Casting|CastToThirdPersonCharacter (Game|GetPlayerCharacter 0))))
  (Variables|Default|SetFuseInside false))

(event EventOnInteract
  (bind _returnvalue (Game|GetPlayerCharacter 0))
  (bind _sm_fuse (Variables|Default|GetSM_Fuse))
  (bind _asthird_person_character (Utilities|Casting|CastToThirdPersonCharacter _returnvalue))
  (if (not (Variables|Default|GetFuseInside))
    (bind _asthird_person_character_2 (Utilities|Casting|CastToThirdPersonCharacter (Game|GetPlayerCharacter 0)))
    (if (Variables|/Game/ThirdPersonBP/Blueprints/ThirdPersonCharacter.ThirdPersonCharacter_C|GetHasFuse _asthird_person_character_2)
      (Variables|/Game/ThirdPersonBP/Blueprints/ThirdPersonCharacter.ThirdPersonCharacter_C|SetHasFuse _asthird_person_character_2 true)
      (Variables|Default|SetFuseInside true)
      (Rendering|SetVisibility _sm_fuse false false)
      (Physics|SetSimulatePhysics _sm_fuse false)
      (Transformation|SetRelativeTransform _sm_fuse (Variables|Default|GetFuseTransform) false)
      (bind _asbp_fuse_standard (Utilities|Casting|CastToBP_FuseStandard (Variables|/Script/Engine.ChildActorComponent|GetChildActor (Variables|Default|GetBP_FuseStandard))))
      (Default|Trigger _asbp_fuse_standard)
      (Utilities|Time|SetTimerbyFunctionName 0 "Fuse Break" (Variables|/Game/ThirdPersonBP/Blueprints/ThirdPersonCharacter.ThirdPersonCharacter_C|GetTimeFuseBreak _asthird_person_character))
      (Default|RemovePlaceFuse _asthird_person_character)
      (Default|StartFuseCountdown _asthird_person_character)
      (Default|AddEscape _asthird_person_character)
      (Default|CallStartCountdown))))

(event EventBeginPlay
  (bind _asbp_fuse_standard (Utilities|Casting|CastToBP_FuseStandard (Variables|/Script/Engine.ChildActorComponent|GetChildActor (Variables|Default|GetBP_FuseStandard))))
  (Default|Trigger _asbp_fuse_standard))

(event Collision|EventActorBeginOverlap
  (params (OtherActor :type Actor%20Object%20Reference)))

(event EventTick
  (params (DeltaSeconds :type Float%20%28single-precision%29)))

(fn ConstructionScript
  (Variables|Default|SetFuseTransform (Transformation|GetRelativeTransform (Variables|Default|GetSM_Fuse))))