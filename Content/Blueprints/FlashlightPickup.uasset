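; Interactable flashlight pickup that gives the third-person character a lamp and introduces the "Get the Flashlight" mission.
; Overlapping its box plays a timeline that slides the WOmanV2 component along Y, then shows the mission widget the first time it finishes.
; Interacting hides the flashlight mesh, zeroes the spotlight, sets HasLamp, removes the widget and activates VentCap.
; It also writes HasLamp into the GameSaveSlot save.
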(event OnComponentBeginOverlap(Box)
  (params (OtherActor :type Actor%20Object%20Reference) (OtherComp :type Primitive%20Component%20Object%20Reference) (OtherBodyIndex :type Integer) (bFromSweep :type Boolean) (SweepResult :type Hit%20Result%20Structure%20%28by%20ref%29))
  (bind _woman_v2 (Variables|Default|GetWOman_v2))
  (bind _relativelocation (Variables|/Script/Engine.SceneComponent|GetRelativeLocation _woman_v2))
  (bind (_x _y _z) (Math|Vector|BreakVector _relativelocation))
  (bind _newtrack_0 (Timeline|Timeline_0 Play)
    (:Update
      (Transformation|SetRelativeLocation _woman_v2 (Math|Vector|MakeVector _x _newtrack_0 _z) false))
    (:Finished
      (if (not (Variables|Default|GetActivated))
        (Variables|Default|SetActivated true)
        (bind _returnvalue (UserInterface|CreateWidget "/Game/Interface/Missions1/GetTheFlashlight.GetTheFlashlight_C"))
        (bind _output_get (Variables|Default|SetMission _returnvalue))
        (UserInterface|Viewport|AddtoViewport _returnvalue 0)))))

(event EventBeginPlay)

(event Collision|EventActorBeginOverlap
  (params (OtherActor :type Actor%20Object%20Reference)))

(event EventTick
  (params (DeltaSeconds :type Float%20%28single-precision%29)))

(event EventOnInteract
  (Rendering|ToggleVisibility (Variables|Default|GetSM_Flashlight) false)
  (Rendering|Components|Light|SetIntensity (Variables|Default|GetSpotLight) 0.0)
  (bind _asthird_person_character (Utilities|Casting|CastToThirdPersonCharacter (Game|GetPlayerCharacter 0)))
  (Variables|/Game/ThirdPersonBP/Blueprints/ThirdPersonCharacter.ThirdPersonCharacter_C|SetHasLamp? _asthird_person_character true)
  (Widget|RemovefromParent (Variables|Default|GetMission))
  (Default|Activate (Variables|Default|GetVentCap))
  (bind _returnvalue (SaveGame|LoadGamefromSlot "GameSaveSlot"))
  (bind _output_get (Variables|Default|SetSaveGameRef _returnvalue))
  (bind _asgame_saver (Utilities|Casting|CastToGameSaver _output_get))
  (Variables|/Game/SaveGame/GameSaver.GameSaver_C|SetHasLamp _asgame_saver true)
  (SaveGame|SaveGametoSlot (Variables|Default|GetSaveGameRef) "GameSaveSlot"))

(fn ConstructionScript)