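; BP_TeddyDoor is an interactable door terminal that controls a child-actor BP_Door and signals whether access is granted.
; OnInteract flashes red with an error sound when Locked, otherwise turns green, plays success audio and triggers the door; OpenDoor bypasses the lock.
; A Timer timeline, played forward or reversed, restores the terminal's blue color when finished.
; The construction script creates the terminal's dynamic material and pre-lowers the inner door when Open.
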(event Custom|Open%20Door
  (Rendering|Material|SetVectorParameterValue (Variables|Default|GetMaterial) "Color" "(R=0.079781,G=0.620000,B=0.096582,A=1.000000)" :!class /Script/Engine.MaterialInstanceDynamic)
  (Class|GameplayStatics|PlaySoundAttached "/Game/Audio/Sounds/SpaceshipInterfaceSuccess_Cue.SpaceshipInterfaceSuccess_Cue" (Variables|Default|GetSM_DoorTerminal))
  (bind _asbp_door (Utilities|Casting|CastToBP_Door (Variables|/Script/Engine.ChildActorComponent|GetChildActor (Variables|Default|GetBP_TestDoor))))
  (Default|TriggerDoor _asbp_door)
  (Timeline|Timer ReverseFromEnd
    (:Finished
      (Rendering|Material|SetVectorParameterValue (Variables|Default|GetMaterial) "Color" "(R=0.376471,G=0.490196,B=1.000000,A=0.000000)" :!class /Script/Engine.MaterialInstanceDynamic))))

(event EventBeginPlay)

(event Collision|EventActorBeginOverlap
  (params (OtherActor :type Actor%20Object%20Reference)))

(event EventTick
  (params (DeltaSeconds :type Float%20%28single-precision%29)))

(event EventOnInteract
  (bind _sm_doorterminal (Variables|Default|GetSM_DoorTerminal))
  (if (Variables|Default|GetLocked?)
    (Rendering|Material|SetVectorParameterValue (Variables|Default|GetMaterial) "Color" "(R=0.600000,G=0.079729,B=0.075000,A=1.000000)" :!class /Script/Engine.MaterialInstanceDynamic)
    (Class|GameplayStatics|PlaySoundAttached "/Game/Audio/Sounds/SpaceshipInterfaceError_Cue.SpaceshipInterfaceError_Cue" _sm_doorterminal)
    (Timeline|Timer PlayFromStart
      (:Finished
        (Rendering|Material|SetVectorParameterValue (Variables|Default|GetMaterial) "Color" "(R=0.376471,G=0.490196,B=1.000000,A=0.000000)" :!class /Script/Engine.MaterialInstanceDynamic)))
    (else
      (Rendering|Material|SetVectorParameterValue (Variables|Default|GetMaterial) "Color" "(R=0.079781,G=0.620000,B=0.096582,A=1.000000)" :!class /Script/Engine.MaterialInstanceDynamic)
      (Class|GameplayStatics|PlaySoundAttached "/Game/Audio/Sounds/SpaceshipInterfaceSuccess_Cue.SpaceshipInterfaceSuccess_Cue" _sm_doorterminal)
      (bind _asbp_door (Utilities|Casting|CastToBP_Door (Variables|/Script/Engine.ChildActorComponent|GetChildActor (Variables|Default|GetBP_TestDoor))))
      (Default|TriggerDoor _asbp_door)
      (Timeline|Timer ReverseFromEnd))))

(fn ConstructionScript
  (bind _returnvalue (Rendering|Material|CreateDynamicMaterialInstance "/Game/General/Sources/DoorTerminal/M_DoorTerminal.M_DoorTerminal" :!class /Script/Engine.KismetMaterialLibrary))
  (bind _output_get (Variables|Default|SetMaterial _returnvalue))
  (Rendering|Material|SetMaterial (Variables|Default|GetSM_DoorTerminal) 0 _output_get)
  (if (Variables|Default|GetOpen?)
    (bind _asbp_door (Utilities|Casting|CastToBP_Door (Variables|/Script/Engine.ChildActorComponent|GetChildActor (Variables|Default|GetBP_TestDoor))))
    (Transformation|SetRelativeLocation (Variables|/Game/Blueprints/BP_Door.BP_Door_C|Getdoor_inner _asbp_door) (Math|Vector|MakeVector (.X (Math|Vector|BreakVector (Variables|/Script/Engine.SceneComponent|GetRelativeLocation (Variables|/Game/Blueprints/BP_Door.BP_Door_C|Getdoor_inner _asbp_door)))) (.Y (Math|Vector|BreakVector (Variables|/Script/Engine.SceneComponent|GetRelativeLocation (Variables|/Game/Blueprints/BP_Door.BP_Door_C|Getdoor_inner _asbp_door)))) -399.0) false)))