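; BP_VentFanFallingOut is a vent fan that switches from a mounted state to a fallen-out state when something overlaps its trigger Box.
; Construction passes on, speed and volume settings to a child BP_Fanrotate, and switches off and hides a second child fan and static mesh.
; On overlap, it hides the frame, disables its collision and swaps visibility to that second fan and mesh, with no filter on the overlapping actor.
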(event OnComponentBeginOverlap(Box)
  (params (OtherActor :type Actor%20Object%20Reference) (OtherComp :type Primitive%20Component%20Object%20Reference) (OtherBodyIndex :type Integer) (bFromSweep :type Boolean) (SweepResult :type Hit%20Result%20Structure%20%28by%20ref%29))
  (Rendering|SetVisibility (Variables|Default|GetSM_FanFrame) false true)
  (Collision|SetCollisionEnabled (Variables|Default|GetSM_FanFrame) "NoCollision")
  (bind _asbp_fanrotate (Utilities|Casting|CastToBP_Fanrotate (Variables|/Script/Engine.ChildActorComponent|GetChildActor (Variables|Default|GetBP_Fanrotate))))
  (Default|Dissappear _asbp_fanrotate)
  (Rendering|SetVisibility (Variables|Default|GetStaticMesh) true true)
  (bind _asbp_fanrotate_2 (Utilities|Casting|CastToBP_Fanrotate (Variables|/Script/Engine.ChildActorComponent|GetChildActor (Variables|Default|GetChildActor))))
  (Default|Appear _asbp_fanrotate_2))

(event EventBeginPlay)

(event Collision|EventActorBeginOverlap
  (params (OtherActor :type Actor%20Object%20Reference)))

(event EventTick
  (params (DeltaSeconds :type Float%20%28single-precision%29)))

(fn ConstructionScript
  (bind _asbp_fanrotate (Utilities|Casting|CastToBP_Fanrotate (Variables|/Script/Engine.ChildActorComponent|GetChildActor (Variables|Default|GetBP_Fanrotate))))
  (Variables|/Game/General/BP_Fanrotate.BP_Fanrotate_C|SetOn? _asbp_fanrotate (Variables|Default|GetOn?))
  (Variables|/Game/General/BP_Fanrotate.BP_Fanrotate_C|SetRotationSpeed _asbp_fanrotate (Variables|Default|GetRoationSpeed))
  (Variables|/Game/General/BP_Fanrotate.BP_Fanrotate_C|SetVolume _asbp_fanrotate (Variables|Default|GetVolume))
  (bind _asbp_fanrotate_2 (Utilities|Casting|CastToBP_Fanrotate (Variables|/Script/Engine.ChildActorComponent|GetChildActor (Variables|Default|GetChildActor))))
  (Variables|/Game/General/BP_Fanrotate.BP_Fanrotate_C|SetOn? _asbp_fanrotate_2 false)
  (Rendering|SetVisibility (Variables|Default|GetStaticMesh) false true)
  (Default|Dissappear _asbp_fanrotate_2))