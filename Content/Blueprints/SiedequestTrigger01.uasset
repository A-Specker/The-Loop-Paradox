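; Side-quest trigger pad that, on first interaction only, toggles Footsteps, opens a linked door and shows a note.
; The construction script tints a dynamic screen material and point light with ScreenColor, and a BeginPlay timeline animates both emissive and light intensity.
; The Note widget takes UI-only input with a visible cursor.
; A second timeline blends in post-processing, which the PPOff event reverses.
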(event Custom|PPOff
  (bind _blend_weight (Timeline|PP ReverseFromEnd)
    (:Update
      (Variables|/Script/Engine.PostProcessComponent|SetBlendWeight (Variables|Default|GetPostProcess) _blend_weight))))

(event EventOnInteract
  (if (not (Variables|Default|GetTriggered))
    (Variables|Default|SetTriggered true)
    (Default|Toggle (Variables|Default|GetFootsteps))
    (Default|OpenDoor (Variables|Default|GetDoor))
    (CallFunction|Read)
    (bind _blend_weight (Timeline|PP Play)
      (:Update
        (Variables|/Script/Engine.PostProcessComponent|SetBlendWeight (Variables|Default|GetPostProcess) _blend_weight)))))

(event EventBeginPlay
  (bind _emissive (Timeline|Timeline_0 Play)
    (:Update
      (Rendering|Material|SetScalarParameterValue (Variables|Default|GetDynamicMaterial) "Emissive" _emissive :!class /Script/Engine.MaterialInstanceDynamic)
      (Rendering|Components|Light|SetIntensity (Variables|Default|GetPointLight) (* _emissive (Variables|Default|GetLightIntensity))))))

(fn ConstructionScript
  (bind _screencolor (Variables|Default|GetScreenColor))
  (bind _returnvalue (Rendering|Material|CreateDynamicMaterialInstance "/Game/General/Sources/Pad/M_Pad.M_Pad" :!class /Script/Engine.KismetMaterialLibrary))
  (bind _output_get (Variables|Default|SetDynamicMaterial _returnvalue))
  (Rendering|Material|SetMaterial (Variables|Default|GetSM_Pad) 0 _output_get)
  (Rendering|Material|SetVectorParameterValue (Variables|Default|GetDynamicMaterial) "ScreenColor" _screencolor :!class /Script/Engine.MaterialInstanceDynamic)
  (Rendering|Components|Light|SetLightColor (Variables|Default|GetPointLight) _screencolor))

(fn Read
  (bind _returnvalue (Game|GetPlayerController 0))
  (bind _returnvalue_2 (UserInterface|CreateWidget (Variables|Default|GetNote)))
  (UserInterface|Viewport|AddtoViewport _returnvalue_2 0)
  (Input|SetInputModeUIOnly _returnvalue _returnvalue_2 true)
  (Variables|/Script/Engine.PlayerController|SetbShowMouseCursor _returnvalue true)
  (Class|Widget|SetUserFocus _returnvalue_2 _returnvalue)
  (return))