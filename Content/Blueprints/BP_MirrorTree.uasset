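; Tree actor that a time gun toggles between young and aged, with two laser beams that can be switched on and off.
; A timeline plays forward or in reverse to drive leaf age and branch darkness on dynamic materials, with falling leaves while aging.
; When it finishes, it flips the Young state and calls CallCheckMirrorAndTree.
; The construction script sets beam endpoints and colors, configuring the second only if both lasers are enabled.
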(event Custom|ToggleLaser1On
  ;[1 1 1] Toggle Laser
  (Variables|Default|SetgotLaser1? true)
  (Rendering|SetVisibility (Variables|Default|GetLaser01) true false))

(event Custom|ToggleLaser1Off
  ;[1 1 1] Toggle Laser
  (Variables|Default|SetgotLaser1? false)
  (Rendering|SetVisibility (Variables|Default|GetLaser01) false false))

(event Custom|ToggleLaser2On
  ;[1 1 1] Toggle Laser
  (Variables|Default|SetgotLaser2? true)
  (Rendering|SetVisibility (Variables|Default|GetLaser02) true false))

(event Custom|ToggleLaser2Off
  ;[1 1 1] Toggle Laser
  (Variables|Default|SetgotLaser2? false)
  (Rendering|SetVisibility (Variables|Default|GetLaser02) false false))

(event EventBeginPlay
  ;[1 1 1] Toggle Off at Beginning
  (CallFunction|ToggleLaser1Off)
  (CallFunction|ToggleLaser2Off)
  (Components|Activation|SetActive (Variables|Default|GetFallingLeafs) false true))

(event EventOnTimeGun
  (params (Location :type Vector :default "0, 0, 0"))
  ;[1 1 1] Aging
  (if (not (Variables|Default|GetAging))
    (if (Variables|Default|GetYoung)
      (Variables|Default|SetAging true)
      (Components|Activation|SetActive (Variables|Default|GetFallingLeafs) true false)
      (bind (_direction _age _darkness _branchdarkness) (Timeline|Timeline_0 PlayFromStart)
        (:Update
          (Rendering|Material|SetScalarParameterValue (Variables|Default|GetLeavesMat) "Age" _age :!class /Script/Engine.MaterialInstanceDynamic)
          (Rendering|Material|SetScalarParameterValue (Variables|Default|GetLeavesMat) "BranchDarkness" _branchdarkness :!class /Script/Engine.MaterialInstanceDynamic)
          (Rendering|Material|SetScalarParameterValue (Variables|Default|GetTreeMat1) "Darkness" _darkness :!class /Script/Engine.MaterialInstanceDynamic)
          (Rendering|Material|SetScalarParameterValue (Variables|Default|GetTreeMat2) "Darkness" _darkness :!class /Script/Engine.MaterialInstanceDynamic))
        (:Finished
          (if (Variables|Default|GetYoung)
            (Components|Activation|SetActive (Variables|Default|GetFallingLeafs) false false)
            (Variables|Default|SetYoung false)
            (Variables|Default|SetAging false)
            (else
              (Variables|Default|SetYoung true)
              (Variables|Default|SetAging false)))
          (Default|CallCheckMirrorandTree)))
      (else
        (Variables|Default|SetAging true)
        (Timeline|Timeline_0 ReverseFromEnd)))))

(fn ConstructionScript
  (bind _tree (Variables|Default|GetTree))
  (bind _laser01 (Variables|Default|GetLaser01))
  (bind _laser02 (Variables|Default|GetLaser02))
  (bind _returnvalue (Rendering|Material|CreateDynamicMaterialInstance "/Game/Foliage/Tree01/Tree_Leaves_Mat_2.Tree_Leaves_Mat_2" :!class /Script/Engine.KismetMaterialLibrary))
  (bind _output_get (Variables|Default|SetLeavesMat _returnvalue))
  (Rendering|Material|SetScalarParameterValue _output_get "Age" 1e+01 :!class /Script/Engine.MaterialInstanceDynamic)
  (bind _returnvalue_2 (Rendering|Material|CreateDynamicMaterialInstance "/Game/Foliage/Tree01/Tree_Branches_Mat.Tree_Branches_Mat" :!class /Script/Engine.KismetMaterialLibrary))
  (bind _output_get_2 (Variables|Default|SetTreeMat1 _returnvalue_2))
  (bind _returnvalue_3 (Rendering|Material|CreateDynamicMaterialInstance "/Game/Foliage/Tree01/Tree_Branches_2_Mat.Tree_Branches_2_Mat" :!class /Script/Engine.KismetMaterialLibrary))
  (bind _output_get_3 (Variables|Default|SetTreeMat2 _returnvalue_3))
  (Rendering|Material|SetMaterial _tree 2 _output_get)
  (Rendering|Material|SetMaterial _tree 0 _output_get_2)
  (Rendering|Material|SetMaterial _tree 1 _output_get_3)
  ;[1 1 1] Laser
  (if (Variables|Default|GetgotLaser1?)
    (Effects|Components|ParticleSystem|SetVectorParameter _laser01 "Target" (Variables|Default|GetEnd1))
    (Effects|Components|ParticleSystem|SetVectorParameter _laser01 "Source" (Variables|Default|GetStart1))
    (Effects|Components|ParticleSystem|SetVectorParameter _laser01 "color" (Math|Conversions|ToVector(LinearColor) (Variables|Default|GetLaserColor1)))
    ;[1 1 1] Laser
    (if (Variables|Default|GetgotLaser2?)
      (Effects|Components|ParticleSystem|SetVectorParameter _laser02 "Target" (Variables|Default|GetEnd2))
      (Effects|Components|ParticleSystem|SetVectorParameter _laser02 "Source" (Variables|Default|GetStart2))
      (Effects|Components|ParticleSystem|SetVectorParameter _laser02 "color" (Math|Conversions|ToVector(LinearColor) (Variables|Default|GetLaserColor2))))))