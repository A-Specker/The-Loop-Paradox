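; BP_GeneratorTriggerable is a generator prop with a spinning element, glowing material and optional hum that winds down when triggered.
; Construction creates a dynamic material and randomizes rotation speed and a sound roll, so only about one in ten generators plays audio.
; Tick spins the element while On is true.
; Trigger clears On and plays a timeline in reverse, driving rotation, emissive, and the sound's volume and pitch.
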(event Custom|Trigger
  (bind _sound (Variables|Default|GetSound))
  (Variables|Default|SetOn? false)
  (bind (_direction _rotation _emissive _volume_pitch) (Timeline|Timeline_0 ReverseFromEnd)
    (:Update
      (Transformation|AddLocalRotation (Variables|Default|GetSM_GeneratorElem) (Class|KismetMathLibrary|MakeRot 0.0 _rotation 0.0) false)
      (Rendering|Material|SetScalarParameterValue (Variables|Default|GetMaterial) "Emmisive" _emissive :!class /Script/Engine.MaterialInstanceDynamic)
      (if (>= (Variables|Default|GetPlaySound) 0.9)
        (Audio|Components|Audio|SetVolumeMultiplier _sound _volume_pitch :!class /Script/Engine.AudioComponent)
        (Audio|Components|Audio|SetPitchMultiplier _sound _volume_pitch)))))

(event EventBeginPlay
  (if (>= (Variables|Default|GetPlaySound) 0.9)
    (bind _returnvalue (Class|GameplayStatics|PlaySoundAttached "/Game/Audio/Generator/Generator_Cue.Generator_Cue" (Variables|Default|GetSM_GeneratorBody)))
    (bind _output_get (Variables|Default|SetSound _returnvalue))
    (Audio|Components|Audio|SetVolumeMultiplier _output_get 0.75 :!class /Script/Engine.AudioComponent)))

(event Collision|EventActorBeginOverlap
  (params (OtherActor :type Actor%20Object%20Reference)))

(event EventTick
  (params (DeltaSeconds :type Float%20%28single-precision%29))
  (if (Variables|Default|GetOn?)
    (Transformation|AddLocalRotation (Variables|Default|GetSM_GeneratorElem) (Class|KismetMathLibrary|MakeRot 0.0 (Variables|Default|GetRotationSpeed) 0.0) false)))

(fn ConstructionScript
  (bind _returnvalue (Rendering|Material|CreateDynamicMaterialInstance "/Game/General/Sources/Generator/M_Generator.M_Generator" :!class /Script/Engine.KismetMaterialLibrary))
  (bind _output_get (Variables|Default|SetMaterial _returnvalue))
  (Rendering|Material|SetMaterial (Variables|Default|GetSM_GeneratorBody) 0 _output_get)
  (Rendering|Material|SetScalarParameterValue (Variables|Default|GetMaterial) "Emmisive" 5.0 :!class /Script/Engine.MaterialInstanceDynamic)
  (Variables|Default|SetRotationSpeed (Math|Random|RandomFloatinRange 2.0 12.0))
  (Variables|Default|SetPlaySound (Math|Random|RandomFloatinRange 0.0 1.0)))