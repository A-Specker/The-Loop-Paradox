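; BP_SlowMoUpgrade is an interactable pickup that extends the player's slow-motion length.
; OnInteract adds AddSlowLength to SlowMoLength on the ThirdPersonCharacter, then writes SlowMoTime to the GameSaver save in GameSaveSlot.
; The saved value adds AddSlowLength again to the already increased length, so it exceeds the live value by that amount.
; After saving, it destroys only the Sphere component, leaving the actor in place.
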(event EventOnInteract
  (bind _asthird_person_character (Utilities|Casting|CastToThirdPersonCharacter (Game|GetPlayerCharacter 0)))
  (Variables|/Game/ThirdPersonBP/Blueprints/ThirdPersonCharacter.ThirdPersonCharacter_C|SetSlowMoLength _asthird_person_character (+ (Variables|/Game/ThirdPersonBP/Blueprints/ThirdPersonCharacter.ThirdPersonCharacter_C|GetSlowMoLength _asthird_person_character) (Variables|Default|GetAddSlowLength)))
  (bind _returnvalue (SaveGame|LoadGamefromSlot "GameSaveSlot"))
  (bind _output_get (Variables|Default|SetSaveGame _returnvalue))
  (bind _asgame_saver (Utilities|Casting|CastToGameSaver _output_get))
  (Variables|/Game/SaveGame/GameSaver.GameSaver_C|SetSlowMoTime _asgame_saver (+ (Variables|/Game/ThirdPersonBP/Blueprints/ThirdPersonCharacter.ThirdPersonCharacter_C|GetSlowMoLength _asthird_person_character) (Variables|Default|GetAddSlowLength)))
  (SaveGame|SaveGametoSlot (Variables|Default|GetSaveGame) "GameSaveSlot")
  (Components|DestroyComponent (Variables|Default|GetSphere)))

(fn ConstructionScript)