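; A generator puzzle actor that toggles between powered and unpowered on the OnTimeGun event, unlocking or locking its child BP_DoorOpen.
; A timeline plays or reverses to drive the element's spin, emissive glow and the looping cue's volume and pitch.
; Once spin-up finishes, Tick keeps the element rotating at a constant speed.
; The construction script positions and locks the door and creates the dynamic material.
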(event EventBeginPlay
  (bind _returnvalue (Class|GameplayStatics|PlaySoundAttached "/Game/Audio/Generator/Generator_Cue.Generator_Cue" (Variables|Default|GetSM_GeneratorBody)))
  (bind _output_get (Variables|Default|SetSound _returnvalue))
  (Audio|Components|Audio|SetVolumeMultiplier _output_get 0.0 :!class /Script/Engine.AudioComponent))

(event Collision|EventActorBeginOverlap
  (params (OtherActor :type Actor%20Object%20Reference)))

(event EventTick
  (params (DeltaSeconds :type Float%20%28single-precision%29))
  (if (Variables|Default|GetOn?)
    (Transformation|AddLocalRotation (Variables|Default|GetSM_GeneratorElem) (Class|KismetMathLibrary|MakeRot 0.0 (Variables|Default|GetRotationSpeed) 0.0) false)))

(event EventOnTimeGun
  (params (Location :type Vector :default "0, 0, 0"))
  (bind _sound (Variables|Default|GetSound))
  (if (Variables|Default|GetLocked)
    (bind _asbp_door_open (Utilities|Casting|CastToBP_DoorOpen (Variables|/Script/Engine.ChildActorComponent|GetChildActor (Variables|Default|GetBP_DoorOpen))))
    (Variables|/Game/Blueprints/BP_DoorOpen.BP_DoorOpen_C|SetLocked? _asbp_door_open false)
    (Variables|Default|SetLocked false)
    (bind (_direction _rotation _emissive _volume_pitch) (Timeline|Timeline_0 Play)
      (:Update
        (Transformation|AddLocalRotation (Variables|Default|GetSM_GeneratorElem) (Class|KismetMathLibrary|MakeRot 0.0 _rotation 0.0) false)
        (Rendering|Material|SetScalarParameterValue (Variables|Default|GetMaterial) "Emmisive" _emissive :!class /Script/Engine.MaterialInstanceDynamic)
        (Audio|Components|Audio|SetVolumeMultiplier _sound _volume_pitch :!class /Script/Engine.AudioComponent)
        (Audio|Components|Audio|SetPitchMultiplier _sound _volume_pitch))
      (:Finished
        (if (not (Variables|Default|GetLocked))
          (Variables|Default|SetOn? true))))
    (else
      (bind _asbp_door_open_2 (Utilities|Casting|CastToBP_DoorOpen (Variables|/Script/Engine.ChildActorComponent|GetChildActor (Variables|Default|GetBP_DoorOpen))))
      (Variables|/Game/Blueprints/BP_DoorOpen.BP_DoorOpen_C|SetLocked? _asbp_door_open_2 true)
      (Variables|Default|SetOn? false)
      (Variables|Default|SetLocked true)
      (Timeline|Timeline_0 Reverse))))

(fn ConstructionScript
  (Transformation|SetRelativeLocation (Variables|Default|GetBP_DoorOpen) (Variables|Default|GetDoorPosition) false)
  (bind _asbp_door_open (Utilities|Casting|CastToBP_DoorOpen (Variables|/Script/Engine.ChildActorComponent|GetChildActor (Variables|Default|GetBP_DoorOpen))))
  (Variables|/Game/Blueprints/BP_DoorOpen.BP_DoorOpen_C|SetLocked? _asbp_door_open true)
  (bind _returnvalue (Rendering|Material|CreateDynamicMaterialInstance "/Game/General/Sources/Generator/M_Generator.M_Generator" :!class /Script/Engine.KismetMaterialLibrary))
  (bind _output_get (Variables|Default|SetMaterial _returnvalue))
  (Rendering|Material|SetMaterial (Variables|Default|GetSM_GeneratorBody) 0 _output_get)
  (Rendering|Material|SetScalarParameterValue (Variables|Default|GetMaterial) "Emmisive" 0.0 :!class /Script/Engine.MaterialInstanceDynamic))