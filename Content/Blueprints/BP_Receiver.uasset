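; BP_Receiver is a Blueprint with a point light that is switched on and off through two custom events.
; Each event sets the PointLight visibility without propagating to children and records the state in IsLightOn.
; The construction script calls ToggleLightOff when IsLightOn is false, applying the off state at construction.
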(event Custom|Toggle_Light_off
  (Rendering|SetVisibility (Variables|Default|GetPointLight) false false)
  (Variables|Default|SetisLightOn? false))

(event Custom|Toggle_Light_on
  (Rendering|SetVisibility (Variables|Default|GetPointLight) true false)
  (Variables|Default|SetisLightOn? true))

(fn ConstructionScript
  (if (not (Variables|Default|GetisLightOn?))
    (CallFunction|ToggleLightOff)))