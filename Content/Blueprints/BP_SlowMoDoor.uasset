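; BP_SlowMoDoor is a one-time door trap with an error terminal, wrapping a child BP_Door flagged as Error at construction.
; Interacting with the terminal plays an error sound and tints its dynamic material red until a timeline finishes.
; The first trigger box overlap shuts the door and records SlowMoDoor01 in an existing GameSaver slot.
; BeginPlay reads that flag and shuts the door again when it differs from Used.
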(event OnComponentBeginOverlap(Box)
  (params (OtherActor :type Actor%20Object%20Reference) (OtherComp :type Primitive%20Component%20Object%20Reference) (OtherBodyIndex :type Integer) (bFromSweep :type Boolean) (SweepResult :type Hit%20Result%20Structure%20%28by%20ref%29))
  (if (not (Variables|Default|GetUsed?))
    (bind _asbp_door (Utilities|Casting|CastToBP_Door (Variables|/Script/Engine.ChildActorComponent|GetChildActor (Variables|Default|GetBP_TestDoor))))
    (Default|ShutDoor _asbp_door)
    (Variables|Default|SetUsed? true)
    (bind _returnvalue (SaveGame|DoesSaveGameExist (Variables|Default|GetGameSaveSlow)))
    (if _returnvalue
      (bind _returnvalue_2 (SaveGame|LoadGamefromSlot (Variables|Default|GetGameSaveSlow)))
      (bind _output_get (Variables|Default|SetSaveGame _returnvalue_2))
      (bind _asgame_saver (Utilities|Casting|CastToGameSaver _output_get))
      (Variables|/Game/SaveGame/GameSaver.GameSaver_C|SetSlowMoDoor01 _asgame_saver true)
      (SaveGame|SaveGametoSlot (Variables|Default|GetSaveGame) (Variables|Default|GetGameSaveSlow)))))

(event EventBeginPlay
  (bind _returnvalue (SaveGame|DoesSaveGameExist (Variables|Default|GetGameSaveSlow)))
  (if _returnvalue
    (bind _returnvalue_2 (SaveGame|LoadGamefromSlot (Variables|Default|GetGameSaveSlow)))
    (bind _output_get (Variables|Default|SetSaveGame _returnvalue_2))
    (bind _asgame_saver (Utilities|Casting|CastToGameSaver _output_get))
    (if (not (Math|Boolean|Equal(Boolean) (Variables|Default|GetUsed?) (Variables|/Game/SaveGame/GameSaver.GameSaver_C|GetSlowMoDoor01 _asgame_saver)))
      (Variables|Default|SetUsed? true)
      (bind _asbp_door (Utilities|Casting|CastToBP_Door (Variables|/Script/Engine.ChildActorComponent|GetChildActor (Variables|Default|GetBP_TestDoor))))
      (Default|ShutDoor _asbp_door))))

(event EventOnInteract
  (Rendering|Material|SetVectorParameterValue (Variables|Default|GetMaterial) "Color" "(R=0.600000,G=0.079729,B=0.075000,A=1.000000)" :!class /Script/Engine.MaterialInstanceDynamic)
  (Class|GameplayStatics|PlaySoundAttached "/Game/Audio/Sounds/SpaceshipInterfaceError_Cue.SpaceshipInterfaceError_Cue" (Variables|Default|GetSM_DoorTerminal))
  (Timeline|Timeline_0 PlayFromStart
    (:Finished
      (Rendering|Material|SetVectorParameterValue (Variables|Default|GetMaterial) "Color" "(R=0.376471,G=0.490196,B=1.000000,A=0.000000)" :!class /Script/Engine.MaterialInstanceDynamic))))

(fn ConstructionScript
  (bind _asbp_door (Utilities|Casting|CastToBP_Door (Variables|/Script/Engine.ChildActorComponent|GetChildActor (Variables|Default|GetBP_TestDoor))))
  (Variables|/Game/Blueprints/BP_Door.BP_Door_C|SetError? _asbp_door true)
  (bind _returnvalue (Rendering|Material|CreateDynamicMaterialInstance "/Game/General/Sources/DoorTerminal/M_DoorTerminal.M_DoorTerminal" :!class /Script/Engine.KismetMaterialLibrary))
  (bind _output_get (Variables|Default|SetMaterial _returnvalue))
  (Rendering|Material|SetMaterial (Variables|Default|GetSM_DoorTerminal) 0 _output_get))