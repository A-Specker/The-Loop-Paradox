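; BP_Attractor is a force volume that pushes the player character along a fixed direction set by its Arrow component.
; Box overlap begin and end events toggle the AddForce flag, without checking which actor triggered them.
; While the flag is set, Tick applies the Arrow's forward vector scaled by Force to player 0's ThirdPersonCharacter movement component, regardless of distance.
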(event OnComponentBeginOverlap(Box)
  (params (OtherActor :type Actor%20Object%20Reference) (OtherComp :type Primitive%20Component%20Object%20Reference) (OtherBodyIndex :type Integer) (bFromSweep :type Boolean) (SweepResult :type Hit%20Result%20Structure%20%28by%20ref%29))
  (Variables|Default|SetAddForce true))

(event OnComponentEndOverlap(Box)
  (params (OtherActor :type Actor%20Object%20Reference) (OtherComp :type Primitive%20Component%20Object%20Reference) (OtherBodyIndex :type Integer))
  (Variables|Default|SetAddForce false))

(event EventBeginPlay)

(event Collision|EventActorBeginOverlap
  (params (OtherActor :type Actor%20Object%20Reference)))

(event EventTick
  (params (DeltaSeconds :type Float%20%28single-precision%29))
  (if (Variables|Default|GetAddForce)
    (bind _asthird_person_character (Utilities|Casting|CastToThirdPersonCharacter (Game|GetPlayerCharacter 0)))
    (Physics|AddForce (Variables|/Script/Engine.Character|GetCharacterMovement _asthird_person_character) (* (Math|Vector|Normalize (Math|Vector|GetForwardVector (Variables|Default|GetArrow))) (Variables|Default|GetForce)))))

(fn ConstructionScript)