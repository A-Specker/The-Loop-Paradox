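; BP_Lift is an interactable lift that closes its doors and triggers a level load.
; On the first interaction only, it closes the doors through a BP_CloseDoors child actor, sets CurrentLevel to 1 on the player's ThirdPersonCharacter, then calls CallLoadLevel.
; A separate openLiftDoors event opens the same child-actor doors.
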(event Custom|openLiftDoors
  (bind _asbp_close_doors (Utilities|Casting|CastToBP_CloseDoors (Variables|/Script/Engine.ChildActorComponent|GetChildActor (Variables|Default|GetBP_CloseDoors))))
  (Default|OpenDoors _asbp_close_doors))

(event EventOnInteract
  (if (not (Variables|Default|GetUsed))
    (Variables|Default|SetUsed true)
    (bind _asbp_close_doors (Utilities|Casting|CastToBP_CloseDoors (Variables|/Script/Engine.ChildActorComponent|GetChildActor (Variables|Default|GetBP_CloseDoors))))
    (Default|CloseDoors _asbp_close_doors)
    (Variables|/Game/ThirdPersonBP/Blueprints/ThirdPersonCharacter.ThirdPersonCharacter_C|SetCurrentLevel (.AsThird%20Person%20Character (Utilities|Casting|CastToThirdPersonCharacter (Game|GetPlayerCharacter 0))) 1)
    (Default|CallLoadLevel)))

(fn ConstructionScript)