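; Slow-motion upgrade pickup for a sidequest that lengthens the player's slow-mo when the sphere is overlapped.
; On first overlap it saves the picked flag and slow-mo time to GameSaveSlot, adding the bonus again to the already increased value.
; It destroys the pickup, then per Generators entry triggers it, calls PPOff and footprint Toggle, and shows a timed upgrade widget.
; BeginPlay removes the pickup if the save marks it collected.
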(event OnComponentBeginOverlap(Sphere)
  (params (OtherActor :type Actor%20Object%20Reference) (OtherComp :type Primitive%20Component%20Object%20Reference) (OtherBodyIndex :type Integer) (bFromSweep :type Boolean) (SweepResult :type Hit%20Result%20Structure%20%28by%20ref%29))
  (if (not (Variables|Default|GetPickedUp))
    (Variables|Default|SetPickedUp true)
    (bind _asthird_person_character (Utilities|Casting|CastToThirdPersonCharacter (Game|GetPlayerCharacter 0)))
    (Variables|/Game/ThirdPersonBP/Blueprints/ThirdPersonCharacter.ThirdPersonCharacter_C|SetSlowMoLength _asthird_person_character (+ (Variables|/Game/ThirdPersonBP/Blueprints/ThirdPersonCharacter.ThirdPersonCharacter_C|GetSlowMoLength _asthird_person_character) (Variables|Default|GetAddSlowLength)))
    (bind _returnvalue (SaveGame|LoadGamefromSlot "GameSaveSlot"))
    (bind _output_get (Variables|Default|SetSaveGame _returnvalue))
    (bind _asgame_saver (Utilities|Casting|CastToGameSaver _output_get))
    (Variables|/Game/SaveGame/GameSaver.GameSaver_C|SetSlowMoTime _asgame_saver (+ (Variables|/Game/ThirdPersonBP/Blueprints/ThirdPersonCharacter.ThirdPersonCharacter_C|GetSlowMoLength _asthird_person_character) (Variables|Default|GetAddSlowLength)))
    (Variables|/Game/SaveGame/GameSaver.GameSaver_C|SetUpgradesOnePicked _asgame_saver true)
    (SaveGame|SaveGametoSlot (Variables|Default|GetSaveGame) "GameSaveSlot")
    (Components|DestroyComponent (Variables|Default|GetUpgradePickup))
    (for _array_element (Variables|Default|GetGenerators)
      (Default|Trigger _array_element)
      (Default|PPOff (Variables|Default|GetSidequestTrigger))
      (Default|Toggle (Variables|Default|GetFootprints))
      (bind _returnvalue_2 (UserInterface|CreateWidget "/Game/Interface/Missions1/SlowMotionUpgraded.SlowMotionUpgraded_C"))
      (UserInterface|Viewport|AddtoViewport _returnvalue_2 0)
      (Utilities|FlowControl|Delay 1e+01)
      (Widget|RemovefromParent _returnvalue_2))))

(event EventBeginPlay
  (bind _returnvalue (SaveGame|LoadGamefromSlot "GameSaveSlot"))
  (bind _output_get (Variables|Default|SetSaveGame _returnvalue))
  (bind _asgame_saver (Utilities|Casting|CastToGameSaver _output_get))
  (if (Variables|/Game/SaveGame/GameSaver.GameSaver_C|GetUpgradesOnePicked _asgame_saver)
    (Variables|Default|SetPickedUp true)
    (Components|DestroyComponent (Variables|Default|GetUpgradePickup))))

(fn ConstructionScript)