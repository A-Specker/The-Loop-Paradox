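; Rotatable mirror for a laser puzzle, which doubles as a laser emitter when flagged.
; A time gun event, gated by usable and busy flags, advances one of eight rotation steps and plays a yaw timeline, calling the mirror check on every update.
; The construction script sets starting orientation, beam parameters and mirror or emitter mesh visibility.
; The laser starts hidden on BeginPlay and is shown or hidden through toggle events.
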(event Custom|ToggleLaserOn
  ;[1 1 1] Toggle
  (Variables|Default|SetgotLaser? true)
  (Rendering|SetVisibility (Variables|Default|GetLaser01) true false))

(event Custom|ToggleLaserOff
  ;[1 1 1] Toggle
  (Variables|Default|SetgotLaser? false)
  (Rendering|SetVisibility (Variables|Default|GetLaser01) false false))

(event EventBeginPlay
  ;[1 1 1] Begin Play
  (CallFunction|ToggleLaserOff))

(event EventOnTimeGun
  (params (Location :type Vector :default "0, 0, 0"))
  ;[1 1 1] Rotate
  (if (not (Variables|Default|GetNotUsable))
    (if (not (Variables|Default|GetBeingUsed))
      (Variables|Default|SetBeingUsed true)
      (Variables|Default|SetRotationAtStart (Transformation|GetWorldRotation (Variables|Default|GetDefaultSceneRoot)))
      (Variables|Default|SetRotation (Math|Integer|%(Integer) (+ (Variables|Default|GetRotation) 1) 8))
      (bind _mirrorrotation (Timeline|RotateMirrorTimeline PlayFromStart)
        (:Update
          (Transformation|SetActorRotation (Class|KismetMathLibrary|MakeRot (.Pitch (Class|KismetMathLibrary|BreakRot (Variables|Default|GetRotationAtStart))) (+ _mirrorrotation (.Yaw (Class|KismetMathLibrary|BreakRot (Variables|Default|GetRotationAtStart)))) (.Roll (Class|KismetMathLibrary|BreakRot (Variables|Default|GetRotationAtStart)))))
          (Default|CallChecktheMirrors)
          (Utilities|FlowControl|Delay 0.6)
          (Variables|Default|SetBeingUsed false))))))

(fn ConstructionScript
  (bind _defaultsceneroot (Variables|Default|GetDefaultSceneRoot))
  (bind _laser01 (Variables|Default|GetLaser01))
  ;[1 1 1] Laser
  (if (Variables|Default|GetgotLaser?)
    (Effects|Components|ParticleSystem|SetVectorParameter _laser01 "Target" (Variables|Default|GetEnd))
    (Effects|Components|ParticleSystem|SetVectorParameter _laser01 "Source" (Variables|Default|GetStart))
    (Effects|Components|ParticleSystem|SetVectorParameter _laser01 "color" (Math|Conversions|ToVector(LinearColor) (Variables|Default|GetLaserColor))))
  ;[1 1 1] Mirror
  (switch int (Variables|Default|GetRotation)
    (:Default
      (Transformation|SetWorldRotation _defaultsceneroot "0,90.000000, 0" false :!label _label))
    (:0
      (goto _label))
    (:1
      (Transformation|SetWorldRotation _defaultsceneroot "0.000000,135.000000,0.000000" false))
    (:2
      (Transformation|SetWorldRotation _defaultsceneroot "0,180.000000, 0" false))
    (:3
      (Transformation|SetWorldRotation _defaultsceneroot "0,225.000000, 0" false))
    (:4
      (Transformation|SetWorldRotation _defaultsceneroot "0,270.000000, 0" false))
    (:5
      (Transformation|SetWorldRotation _defaultsceneroot "0,315.000000, 0" false))
    (:6
      (Transformation|SetWorldRotation _defaultsceneroot "0,0.000000, 0" false))
    (:7
      (Transformation|SetWorldRotation _defaultsceneroot "0,45.000000, 0" false)))
  (Transformation|AddWorldRotation (Variables|Default|GetDefaultSceneRoot) "0,0.000000, 0" false)
  ;[1 1 1] Emitter
  (if (Variables|Default|GetisEmitter?)
    (Rendering|SetVisibility (Variables|Default|GetCube) false false)
    (Rendering|SetVisibility (Variables|Default|GetCube1) false false)
    (else
      (Rendering|SetVisibility (Variables|Default|GetSM_Emmitter) false false))))