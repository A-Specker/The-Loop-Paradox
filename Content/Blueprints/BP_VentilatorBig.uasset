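; BP_VentilatorBig is a ventilator actor that hosts a BP_Fanrotate child actor.
; On BeginPlay it casts the child actor and calls its Switch function once, presumably to start the fan.
; The construction script sets the child component's relative scale to the inverse of the root's world scale, cancelling any scaling applied to the ventilator.
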(event EventBeginPlay
  (bind _asbp_fanrotate (Utilities|Casting|CastToBP_Fanrotate (Variables|/Script/Engine.ChildActorComponent|GetChildActor (Variables|Default|GetBP_Fanrotate))))
  (Default|Switch _asbp_fanrotate))

(fn ConstructionScript
  (bind _defaultsceneroot (Variables|Default|GetDefaultSceneRoot))
  (bind _returnvalue (Transformation|GetWorldScale _defaultsceneroot))
  (bind (_x _y _z) (Math|Vector|BreakVector _returnvalue))
  (Transformation|SetRelativeScale3D (Variables|Default|GetBP_Fanrotate) (Math|Vector|MakeVector (/ 1.0 _x) (/ 1.0 _y) (/ 1.0 _z))))