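; BP_Pickable is a component that makes its owning actor hover while inside a ventilator.
; On BeginPlay it caches the owner's first primitive component and enables overlap events, and the OnVentilator event toggles the Ventilated state.
; While ventilated, Tick traces downward and pushes along the hit normal with a force that fades linearly over the trace length, setting linear and angular damping on each hit.
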(event EventTick
  (params (DeltaSeconds :type Float%20%28single-precision%29))
  (bind _primitive_component (Variables|Default|GetPrimitive%20Component))
  (bind _returnvalue (Transformation|GetWorldLocation _primitive_component))
  ;[1 1 1] Hovering when Ventilated
  (if (Variables|Default|GetVentilated?)
    (bind (_outhit _returnvalue_2) (Collision|LineTraceByChannel _returnvalue (- _returnvalue (Math|Vector|MakeVector 0.0 0.0 (Variables|Default|GetTraceLength))) "TraceTypeQuery1" false 0 "None"))
    (if _returnvalue_2
      (Physics|AddForce (Variables|Default|GetPrimitive%20Component) (* (.Normal (Collision|BreakHitResult _outhit)) (Math|Float|Lerp 5e+05 0.0 (/ (Math|Vector|VectorLength (- (.Location (Collision|BreakHitResult _outhit)) (Transformation|GetWorldLocation (Variables|Default|GetPrimitive%20Component)))) (Variables|Default|GetTraceLength)))) "None" false)
      (Class|PrimitiveComponent|SetLinearDamping (Variables|Default|GetPrimitive%20Component) 0.6)
      (Class|PrimitiveComponent|SetAngularDamping (Variables|Default|GetPrimitive%20Component) 0.2))))

(event EventBeginPlay
  ;[1 1 1] Get Parent Component
  (bind _output_get (Variables|Default|SetPrimitive%20Component (Utilities|Array|Get(acopy) (Actor|GetComponentsByClass (Components|GetOwner) "/Script/Engine.PrimitiveComponent"))))
  (Variables|/Script/Engine.PrimitiveComponent|SetbGenerateOverlapEvents _output_get true))

(event EventOnVentilator
  ;[1 1 1] Fly when in Ventilator
  (if (Variables|Default|GetVentilated?)
    (Variables|Default|SetVentilated? false)
    (else
      (Variables|Default|SetVentilated? true))))