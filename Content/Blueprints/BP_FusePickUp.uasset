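; BP_FusePickUp is an interactable fuse the player picks up as part of the main quest.
; On interact, if the ThirdPersonCharacter has no fuse, it fires the PickedUpFuse dispatcher and sets HasFuse.
; It writes the fuse flag and quest stage into the GameSaveSlot save immediately.
; It then hides the mesh rather than destroying the actor and swaps the character's fuse mission for the place-fuse objective.
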(event EventOnInteract
  (bind _returnvalue (Game|GetPlayerCharacter 0))
  (bind _asthird_person_character (Utilities|Casting|CastToThirdPersonCharacter _returnvalue))
  (bind _asthird_person_character_2 (Utilities|Casting|CastToThirdPersonCharacter (Game|GetPlayerCharacter 0)))
  (if (not (Variables|/Game/ThirdPersonBP/Blueprints/ThirdPersonCharacter.ThirdPersonCharacter_C|GetHasFuse _asthird_person_character_2))
    (Default|CallPickedUpFuse)
    (bind _asthird_person_character_3 (Utilities|Casting|CastToThirdPersonCharacter (Game|GetPlayerCharacter 0)))
    (Variables|/Game/ThirdPersonBP/Blueprints/ThirdPersonCharacter.ThirdPersonCharacter_C|SetHasFuse _asthird_person_character_3 true)
    (bind _returnvalue_2 (SaveGame|LoadGamefromSlot "GameSaveSlot"))
    (bind _output_get (Variables|Default|SetSaveGame _returnvalue_2))
    (bind _asgame_saver (Utilities|Casting|CastToGameSaver _output_get))
    (Variables|/Game/SaveGame/GameSaver.GameSaver_C|SetGotFuse _asgame_saver true)
    (Variables|/Game/SaveGame/GameSaver.GameSaver_C|SetMainQuest1 _asgame_saver 2)
    (SaveGame|SaveGametoSlot (Variables|Default|GetSaveGame) "GameSaveSlot")
    (Rendering|SetVisibility (Variables|Default|GetStaticMesh) false true)
    (Default|RemoveFuseMission _asthird_person_character)
    (Default|AddPlaceFuse _asthird_person_character)))

(event EventBeginPlay)

(event Collision|EventActorBeginOverlap
  (params (OtherActor :type Actor%20Object%20Reference)))

(event EventTick
  (params (DeltaSeconds :type Float%20%28single-precision%29)))

(fn ConstructionScript)