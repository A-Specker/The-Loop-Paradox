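; BP_AudioLog is an interactable pad with a blinking screen and light, tinted by a configurable color.
; Construction creates the dynamic screen material, and a timeline pulses its emissive and the point light.
; Interacting opens a Note widget, pauses the game and raises post-process blend until the widget closes.
; When flagged as a mission, it can add the fuse mission once and save main quest progress to GameSaveSlot.
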(event EventBeginPlay
  (bind _emissive (Timeline|Blinker Play)
    (:Update
      (Rendering|Material|SetScalarParameterValue (Variables|Default|GetDynamicMaterial) "Emissive" _emissive :!class /Script/Engine.MaterialInstanceDynamic)
      (Rendering|Components|Light|SetIntensity (Variables|Default|GetPointLight) (* _emissive (Variables|Default|GetLightIntesity))))))

(event EventTick
  (params (DeltaSeconds :type Float%20%28single-precision%29))
  (if (Variables|Default|GetOn)
    (if (not (UserInterface|Viewport|IsinViewport (Variables|Default|GetWidget)))
      (Variables|/Script/Engine.PostProcessComponent|SetBlendWeight (Variables|Default|GetPostProcess) 0.0))))

(event EventOnInteract
  (bind _returnvalue (Game|GetPlayerController 0))
  (Variables|Default|SetOn true)
  (Default|CallClicked)
  (bind _returnvalue_2 (UserInterface|CreateWidget (Variables|Default|GetNote)))
  (bind _output_get (Variables|Default|SetWidget _returnvalue_2))
  (UserInterface|Viewport|AddtoViewport _returnvalue_2 0)
  (Input|SetInputModeUIOnly _returnvalue _output_get true)
  (Variables|/Script/Engine.PlayerController|SetbShowMouseCursor _returnvalue true)
  (Class|Widget|SetUserFocus _returnvalue_2 _returnvalue)
  (Game|SetGamePaused true)
  (Variables|/Script/Engine.PostProcessComponent|SetBlendWeight (Variables|Default|GetPostProcess) 1.0)
  (if (Variables|Default|GetMission?)
    (switch int (Variables|Default|GetMission)
      (:0
        (Default|AddFuseMission (.AsThird%20Person%20Character (Utilities|Casting|CastToThirdPersonCharacter (Game|GetPlayerCharacter 0))))
        (Variables|Default|SetMission? false)
        (bind _returnvalue_3 (SaveGame|LoadGamefromSlot "GameSaveSlot"))
        (bind _output_get_2 (Variables|Default|SetSaveGame _returnvalue_3))
        (bind _asgame_saver (Utilities|Casting|CastToGameSaver _output_get_2))
        (Variables|/Game/SaveGame/GameSaver.GameSaver_C|SetMainQuest1 _asgame_saver 1)
        (SaveGame|SaveGametoSlot (Variables|Default|GetSaveGame) "GameSaveSlot")))))

(fn ConstructionScript
  (bind _screencolor (Variables|Default|GetScreenColor))
  (bind _pointlight (Variables|Default|GetPointLight))
  (bind _returnvalue (Rendering|Material|CreateDynamicMaterialInstance "/Game/General/Sources/Pad/M_Pad.M_Pad" :!class /Script/Engine.KismetMaterialLibrary))
  (bind _output_get (Variables|Default|SetDynamicMaterial _returnvalue))
  (Rendering|Material|SetMaterial (Variables|Default|GetSM_Pad) 0 _output_get)
  (Rendering|Material|SetVectorParameterValue (Variables|Default|GetDynamicMaterial) "ScreenColor" _screencolor :!class /Script/Engine.MaterialInstanceDynamic)
  (Rendering|Components|Light|SetLightColor _pointlight _screencolor)
  (Rendering|Components|Light|SetIntensity _pointlight (Variables|Default|GetLightIntesity)))