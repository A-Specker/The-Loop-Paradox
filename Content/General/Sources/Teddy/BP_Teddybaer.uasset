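; Collectible teddy bear for a four-part secret quest, with ColorBear selecting its material and save index.
; Interacting shows the player's teddy widget, increments the count, saves progress to GameSaver and removes the Teddy component.
; The fourth pickup ends the quest, plays a sound, opens the linked door and briefly shows a SecretUnlocked widget.
; On BeginPlay, the Teddy component is destroyed if the save marks it picked.
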(event EventBeginPlay
  (bind _returnvalue (SaveGame|LoadGamefromSlot "GameSaveSlot"))
  (bind _output_get (Variables|Default|SetSaveGame _returnvalue))
  (bind _asgame_saver (Utilities|Casting|CastToGameSaver _output_get))
  (if (Utilities|Array|Get(acopy) (Variables|/Game/SaveGame/GameSaver.GameSaver_C|GetTeddiesPicked _asgame_saver) (Variables|Default|GetcolorBear))
    (Components|DestroyComponent (Variables|Default|GetTeddy))))

(event EventOnInteract
  (bind _asthird_person_character (Utilities|Casting|CastToThirdPersonCharacter (Game|GetPlayerCharacter 0)))
  (if (UserInterface|Viewport|IsinViewport (Variables|/Game/ThirdPersonBP/Blueprints/ThirdPersonCharacter.ThirdPersonCharacter_C|GetTeddyWidget _asthird_person_character))
    _
    (else
      (UserInterface|Viewport|AddtoViewport (Variables|/Game/ThirdPersonBP/Blueprints/ThirdPersonCharacter.ThirdPersonCharacter_C|GetTeddyWidget _asthird_person_character) 0)))
  (Variables|/Game/ThirdPersonBP/Blueprints/ThirdPersonCharacter.ThirdPersonCharacter_C|SetcountCollectedTeddys _asthird_person_character (+ (Variables|/Game/ThirdPersonBP/Blueprints/ThirdPersonCharacter.ThirdPersonCharacter_C|GetcountCollectedTeddys _asthird_person_character) 1))
  (bind _returnvalue (SaveGame|LoadGamefromSlot "GameSaveSlot"))
  (bind _output_get (Variables|Default|SetSaveGame _returnvalue))
  (bind _asgame_saver (Utilities|Casting|CastToGameSaver _output_get))
  (Variables|/Game/SaveGame/GameSaver.GameSaver_C|SetNumTeddies _asgame_saver (Variables|/Game/ThirdPersonBP/Blueprints/ThirdPersonCharacter.ThirdPersonCharacter_C|GetcountCollectedTeddys (.AsThird%20Person%20Character (Utilities|Casting|CastToThirdPersonCharacter (Game|GetPlayerCharacter 0)))))
  (Utilities|Array|SetArrayElem (Variables|/Game/SaveGame/GameSaver.GameSaver_C|GetTeddiesPicked _asgame_saver) (Variables|Default|GetcolorBear) true true)
  (Variables|/Game/SaveGame/GameSaver.GameSaver_C|SetTeddyQuest _asgame_saver true)
  (SaveGame|SaveGametoSlot (Variables|Default|GetSaveGame) "GameSaveSlot")
  (if (== (Variables|/Game/ThirdPersonBP/Blueprints/ThirdPersonCharacter.ThirdPersonCharacter_C|GetcountCollectedTeddys _asthird_person_character) 4)
    (bind _returnvalue_2 (SaveGame|LoadGamefromSlot "GameSaveSlot"))
    (bind _output_get_2 (Variables|Default|SetSaveGame _returnvalue_2))
    (bind _asgame_saver_2 (Utilities|Casting|CastToGameSaver _output_get_2))
    (Variables|/Game/SaveGame/GameSaver.GameSaver_C|SetTeddyQuest _asgame_saver_2 false)
    (SaveGame|SaveGametoSlot _output_get_2 "GameSaveSlot")
    (bind _returnvalue_3 (Class|GameplayStatics|PlaySoundAttached "/Game/Audio/Sounds/DoorSlideOpen_Cue.DoorSlideOpen_Cue" (Variables|Default|GetTeddy)))
    (Audio|Components|Audio|SetVolumeMultiplier _returnvalue_3 2.0 :!class /Script/Engine.AudioComponent)
    (Default|OpenDoor (Variables|Default|GetDoorOpen))
    (bind _asthird_person_character_2 (Utilities|Casting|CastToThirdPersonCharacter (Game|GetPlayerCharacter 0)))
    (Default|RemoveTeddieMission _asthird_person_character_2)
    (bind _returnvalue_4 (UserInterface|CreateWidget "/Game/Interface/Missions1/SecretUnlocked.SecretUnlocked_C"))
    (UserInterface|Viewport|AddtoViewport _returnvalue_4 0))
  (Components|DestroyComponent (Variables|Default|GetTeddy))
  (Utilities|FlowControl|Delay 1e+01)
  (Widget|RemovefromParent _returnvalue_4))

(fn ConstructionScript
  (bind _teddy (Variables|Default|GetTeddy))
  (switch int (Variables|Default|GetcolorBear)
    (:Default
      (Rendering|Material|SetMaterial _teddy 0 "/Game/General/Sources/Teddy/M_teddy1.M_Teddy1" :!label _label))
    (:0
      (goto _label))
    (:1
      (Rendering|Material|SetMaterial _teddy 0 "/Game/General/Sources/Teddy/M_Teddy2.M_Teddy2"))
    (:2
      (Rendering|Material|SetMaterial _teddy 0 "/Game/General/Sources/Teddy/M_Teddy3.M_Teddy3"))
    (:3
      (Rendering|Material|SetMaterial _teddy 0 "/Game/General/Sources/Teddy/M_Teddy4.M_Teddy4"))))