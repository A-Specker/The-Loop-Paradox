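; BP_Fanrotate is a switchable ventilator fan actor that spins a mesh and plays an attached vent sound.
; Switch toggles On and plays or reverses the VentilatorSpeedUp timeline, which drives RotatingMovement yaw plus the sound's volume and pitch.
; Construction Script and BeginPlay set full spin when On; the BeginPlay sound is not stored in VentSound, unlike Switch's.
; Appear and Dissappear only toggle the mesh's collision.
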(event Custom|Appear
  (Collision|SetCollisionEnabled (Variables|Default|GetStaticMesh) "QueryAndPhysics"))

(event Custom|Dissappear
  (Collision|SetCollisionEnabled (Variables|Default|GetStaticMesh) "NoCollision"))

(event Custom|Switch
  (if (Variables|Default|GetOn?)
    (Variables|Default|SetOn? false)
    (bind _animation (Timeline|VentilatorSpeedUp Reverse)
      (:Update
        (Variables|/Script/Engine.RotatingMovementComponent|SetRotationRate (Variables|Default|GetRotatingMovement) (Class|KismetMathLibrary|MakeRot 0.0 (* (Class|KismetMathLibrary|MapRange _animation 0.0 1.0 0.0 (Variables|Default|GetRotationSpeed)) -1.0) 0.0))
        (Audio|Components|Audio|SetVolumeMultiplier (Variables|Default|GetVentSound) _animation :!class /Script/Engine.AudioComponent)
        (Audio|Components|Audio|SetPitchMultiplier (Variables|Default|GetVentSound) (Class|KismetMathLibrary|MapRange _animation 0.0 1.0 0.8 1.0))))
    (else
      (Variables|Default|SetOn? true)
      (bind _returnvalue (Class|GameplayStatics|PlaySoundAttached "/Game/Audio/Sounds/VentVentilator_Cue.VentVentilator_Cue" (Variables|Default|GetStaticMesh)))
      (Variables|Default|SetVentSound _returnvalue)
      (Timeline|VentilatorSpeedUp Play))))

(event EventBeginPlay
  (if (Variables|Default|GetOn?)
    (bind _returnvalue (Class|GameplayStatics|PlaySoundAttached "/Game/Audio/Sounds/VentVentilator_Cue.VentVentilator_Cue" (Variables|Default|GetStaticMesh)))
    (Audio|Components|Audio|AdjustVolume _returnvalue 0.0 (Variables|Default|GetVolume) :!class /Script/Engine.AudioComponent)
    (if (Variables|Default|GetOn?)
      (Variables|/Script/Engine.RotatingMovementComponent|SetRotationRate (Variables|Default|GetRotatingMovement) (Class|KismetMathLibrary|MakeRot 0.0 (* (Variables|Default|GetRotationSpeed) -1.0) 0.0))
      (Variables|Default|SetPreviousRotationSpeed (Variables|Default|GetRotationSpeed)))))

(event Collision|EventActorBeginOverlap
  (params (OtherActor :type Actor%20Object%20Reference)))

(event EventTick
  (params (DeltaSeconds :type Float%20%28single-precision%29)))

(fn ConstructionScript
  (if (Variables|Default|GetOn?)
    (Variables|/Script/Engine.RotatingMovementComponent|SetRotationRate (Variables|Default|GetRotatingMovement) (Class|KismetMathLibrary|MakeRot 0.0 (* (Variables|Default|GetRotationSpeed) -1.0) 0.0))
    (Variables|Default|SetPreviousRotationSpeed (Variables|Default|GetRotationSpeed))))