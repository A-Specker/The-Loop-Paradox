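; Rotating fan hazard that kills the player character on a component hit.
; When On, it spins via RotatingMovement at negative RotationSpeed yaw, set in the construction script and at BeginPlay, which also attaches a loud turbine sound.
; Any hit on the fan mesh calls Death on player 0's ThirdPersonCharacter, without checking what struck it.
; The Switch event is an empty stub.
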(event OnComponentHit(SM_FanKill)
  (params (OtherActor :type Actor%20Object%20Reference) (OtherComp :type Primitive%20Component%20Object%20Reference) (NormalImpulse :type Vector :default "0, 0, 0") (Hit :type Hit%20Result%20Structure%20%28by%20ref%29))
  (bind _asthird_person_character (Utilities|Casting|CastToThirdPersonCharacter (Game|GetPlayerCharacter 0)))
  (Default|Death _asthird_person_character))

(event Custom|Switch)

(event EventBeginPlay
  (if (Variables|Default|GetOn?)
    (Class|GameplayStatics|PlaySoundAttached "/Game/Audio/Sounds/Turbine_LoudCue.Turbine_LoudCue" (Variables|Default|GetSM_FanKill) "None" "0, 0, 0" "KeepRelativeOffset" true)
    (if (Variables|Default|GetOn?)
      (Variables|/Script/Engine.RotatingMovementComponent|SetRotationRate (Variables|Default|GetRotatingMovement) (Class|KismetMathLibrary|MakeRot 0.0 (* (Variables|Default|GetRotationSpeed) -1.0) 0.0))
      (Variables|Default|SetPreviousRotationSpeed (Variables|Default|GetRotationSpeed)))))

(fn ConstructionScript
  (if (Variables|Default|GetOn?)
    (Variables|/Script/Engine.RotatingMovementComponent|SetRotationRate (Variables|Default|GetRotatingMovement) (Class|KismetMathLibrary|MakeRot 0.0 (* (Variables|Default|GetRotationSpeed) -1.0) 0.0))
    (Variables|Default|SetPreviousRotationSpeed (Variables|Default|GetRotationSpeed))))