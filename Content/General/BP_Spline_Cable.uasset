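; BP_Spline_Cable is a construction-time actor that builds a cable from spline meshes along an editable spline.
; The construction script adds one spline mesh per segment, attached to TopScene, using neighboring points' local positions and tangents.
; Each segment's start is pushed back along its tangent by PlugAmount to plug the ends together.
; A non-uniform scale warning using a dynamic material is disconnected, and the event graph is empty.
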(event EventBeginPlay)

(event Collision|EventActorBeginOverlap
  (params (OtherActor :type Actor%20Object%20Reference)))

(event EventTick
  (params (DeltaSeconds :type Float%20%28single-precision%29)))

(fn ConstructionScript
  (bind _spline (Variables|Default|GetSpline))
  ;[1 1 1] If 3 Splines -> 2 Meshes#
  (for _index (range 0 (- (Class|SplineComponent|GetNumSplinePoints) 2))
    ;[1 1 1] Add Spline Object and Connect it
    (bind _returnvalue (AddComponent|AddSplineMeshComponent true))
    (Class|SceneComponent|Attachto _returnvalue (Variables|Default|GetTopScene) "None" "KeepRelativeOffset" true)
    (SplineMesh|SetStartandEnd _returnvalue (- (.LocalLocation (Class|SplineComponent|GetLocalLocationandTangentatSplinePoint _spline _index)) (* (Math|Vector|Normalize (.LocalTangent (Class|SplineComponent|GetLocalLocationandTangentatSplinePoint _spline _index))) (Variables|Default|GetPlugAmount))) (.LocalTangent (Class|SplineComponent|GetLocalLocationandTangentatSplinePoint _spline _index)) (.LocalLocation (Class|SplineComponent|GetLocalLocationandTangentatSplinePoint _spline (+ _index 1))) (.LocalTangent (Class|SplineComponent|GetLocalLocationandTangentatSplinePoint _spline (+ _index 1))) :!class /Script/Engine.SplineMeshComponent)))