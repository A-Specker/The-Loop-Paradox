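; BP_BooksClosed is a closed book prop actor that gets a random look each time it is constructed.
; Its construction script creates a dynamic instance of M_BookClosed, sets a random RGB BookColor and a random Brightness, and applies it to the book mesh.
; The event graph holds no logic.
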(event EventBeginPlay)

(event Collision|EventActorBeginOverlap
  (params (OtherActor :type Actor%20Object%20Reference)))

(event EventTick
  (params (DeltaSeconds :type Float%20%28single-precision%29)))

(fn ConstructionScript
  (bind _returnvalue (Rendering|Material|CreateDynamicMaterialInstance "/Game/General/Sources/BookClosed/M_BookClosed.M_BookClosed" :!class /Script/Engine.KismetMaterialLibrary))
  (bind _output_get (Variables|Default|SetBookMaterial _returnvalue))
  (Rendering|Material|SetVectorParameterValue _output_get "BookColor" (Utilities|Struct|MakeLinearColor (Math|Random|RandomFloatinRange 0.0 1.0) (Math|Random|RandomFloatinRange 0.0 1.0) (Math|Random|RandomFloatinRange 0.0 1.0) 0.0) :!class /Script/Engine.MaterialInstanceDynamic)
  (Rendering|Material|SetScalarParameterValue _output_get "Brightness" (Math|Random|RandomFloatinRange 3.0 8.0) :!class /Script/Engine.MaterialInstanceDynamic)
  (Rendering|Material|SetMaterial (Variables|Default|GetSM_BookClosed) 0 (Variables|Default|GetBookMaterial)))