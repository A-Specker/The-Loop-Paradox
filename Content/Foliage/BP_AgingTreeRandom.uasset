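; Foliage tree actor that toggles between young and aged looks when AgeTree or OnTimeGun fires, ignoring triggers while a transition runs.
; The construction script builds one of three scaled meshes and one of five particle systems from TreeNumber and ParticleNumber, then applies dynamic leaf and branch materials.
; A timeline plays forward or in reverse to drive material age and darkness, with particles active during the young-to-aged transition until a stop event.
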(event Custom|AgeTree
  (if (not (Variables|Default|GetAging))
    (if (Variables|Default|GetYoung)
      (Variables|Default|SetAging true)
      (Components|Activation|SetActive (Variables|Default|GetParticleSystem) true false)
      (bind (_direction _age _darkness _branchdarkness) (Timeline|Timeline_0 PlayFromStart)
        (:Update
          (Rendering|Material|SetScalarParameterValue (Variables|Default|GetLeavesMat) "Age" _age :!class /Script/Engine.MaterialInstanceDynamic)
          (Rendering|Material|SetScalarParameterValue (Variables|Default|GetLeavesMat) "BranchDarkness" _branchdarkness :!class /Script/Engine.MaterialInstanceDynamic)
          (Rendering|Material|SetScalarParameterValue (Variables|Default|GetTreeMat1) "Darkness" _darkness :!class /Script/Engine.MaterialInstanceDynamic)
          (Rendering|Material|SetScalarParameterValue (Variables|Default|GetTreeMat2) "Darkness" _darkness :!class /Script/Engine.MaterialInstanceDynamic))
        (:Finished
          (if (Variables|Default|GetYoung)
            (Variables|Default|SetYoung false)
            (else
              (Variables|Default|SetYoung true)))
          (Variables|Default|SetAging false))
        (:ParticleStop
          (if (Variables|Default|GetYoung)
            (Components|Activation|SetActive (Variables|Default|GetParticleSystem) false false))))
      (else
        (Variables|Default|SetAging true)
        (Timeline|Timeline_0 ReverseFromEnd)))))

(event EventBeginPlay
  (Components|Activation|SetActive (Variables|Default|GetParticleSystem) false true))

(event Collision|EventActorBeginOverlap
  (params (OtherActor :type Actor%20Object%20Reference)))

(event EventTick
  (params (DeltaSeconds :type Float%20%28single-precision%29)))

(event EventOnTimeGun
  (params (Location :type Vector :default "0, 0, 0"))
  (if (not (Variables|Default|GetAging))
    (if (Variables|Default|GetYoung)
      (Variables|Default|SetAging true)
      (Components|Activation|SetActive (Variables|Default|GetParticleSystem) true false)
      (bind (_direction _age _darkness _branchdarkness) (Timeline|Timeline_0 PlayFromStart)
        (:Update
          (Rendering|Material|SetScalarParameterValue (Variables|Default|GetLeavesMat) "Age" _age :!class /Script/Engine.MaterialInstanceDynamic)
          (Rendering|Material|SetScalarParameterValue (Variables|Default|GetLeavesMat) "BranchDarkness" _branchdarkness :!class /Script/Engine.MaterialInstanceDynamic)
          (Rendering|Material|SetScalarParameterValue (Variables|Default|GetTreeMat1) "Darkness" _darkness :!class /Script/Engine.MaterialInstanceDynamic)
          (Rendering|Material|SetScalarParameterValue (Variables|Default|GetTreeMat2) "Darkness" _darkness :!class /Script/Engine.MaterialInstanceDynamic))
        (:Finished
          (if (Variables|Default|GetYoung)
            (Variables|Default|SetYoung false)
            (else
              (Variables|Default|SetYoung true)))
          (Variables|Default|SetAging false))
        (:ParticleStop
          (if (Variables|Default|GetYoung)
            (Components|Activation|SetActive (Variables|Default|GetParticleSystem) false false))))
      (else
        (Variables|Default|SetAging true)
        (Timeline|Timeline_0 ReverseFromEnd)))))

(fn ConstructionScript
  (bind _tree01mult (Variables|Default|GetTree01Mult))
  (bind _tree02mult (Variables|Default|GetTree02Mult))
  (bind _tree03mult (Variables|Default|GetTree03Mult))
  (bind _tree_size (Variables|Default|GetTree%20Size))
  (bind _returnvalue (* _tree_size _tree03mult))
  (bind _returnvalue_2 (* _tree01mult _tree_size))
  (bind _returnvalue_3 (* _tree_size _tree02mult))
  (switch int (Variables|Default|GetTreeNumber)
    (:0
      (bind _returnvalue_4 (AddComponent|AddStaticMeshComponent false (Math|Transform|MakeTransform "0, 0, 0" "0, 0, 0" (Math|Vector|MakeVector _returnvalue_2 _returnvalue_2 _returnvalue_2))))
      (Variables|Default|SetTree _returnvalue_4))
    (:1
      (bind _returnvalue_5 (AddComponent|AddStaticMeshComponent false (Math|Transform|MakeTransform "0, 0, 0" "0, 0, 0" (Math|Vector|MakeVector _returnvalue_3 _returnvalue_3 _returnvalue_3))))
      (Variables|Default|SetTree _returnvalue_5))
    (:2
      (bind _returnvalue_6 (AddComponent|AddStaticMeshComponent false (Math|Transform|MakeTransform "0, 0, 0" "0, 0, 0" (Math|Vector|MakeVector _returnvalue _returnvalue _returnvalue))))
      (Variables|Default|SetTree _returnvalue_6)))
  (CallFunction|ApplyMaterial (Variables|Default|GetTree))
  (switch int (Variables|Default|GetParticleNumber)
    (:Default
      (bind _returnvalue_7 (AddComponent|AddParticleSystemComponent false :!label _label))
      (Variables|Default|SetParticleSystem _returnvalue_7))
    (:0
      (goto _label))
    (:1
      (bind _returnvalue_8 (AddComponent|AddParticleSystemComponent false))
      (Variables|Default|SetParticleSystem _returnvalue_8))
    (:2
      (bind _returnvalue_9 (AddComponent|AddParticleSystemComponent false))
      (Variables|Default|SetParticleSystem _returnvalue_9))
    (:3
      (bind _returnvalue_10 (AddComponent|AddParticleSystemComponent false))
      (Variables|Default|SetParticleSystem _returnvalue_10))
    (:4
      (bind _returnvalue_11 (AddComponent|AddParticleSystemComponent false))
      (Variables|Default|SetParticleSystem _returnvalue_11))))

(fn ApplyMaterial
  (params (Tree :type Primitive%20Component%20Object%20Reference))
  (bind _returnvalue (Rendering|Material|CreateDynamicMaterialInstance "/Game/Foliage/Tree01/Tree_Leaves_Mat_2.Tree_Leaves_Mat_2" :!class /Script/Engine.KismetMaterialLibrary))
  (bind _output_get (Variables|Default|SetLeavesMat _returnvalue))
  (Rendering|Material|SetScalarParameterValue _output_get "Age" 1e+01 :!class /Script/Engine.MaterialInstanceDynamic)
  (bind _returnvalue_2 (Rendering|Material|CreateDynamicMaterialInstance "/Game/Foliage/Tree01/Tree_Branches_Mat.Tree_Branches_Mat" :!class /Script/Engine.KismetMaterialLibrary))
  (bind _output_get_2 (Variables|Default|SetTreeMat1 _returnvalue_2))
  (bind _returnvalue_3 (Rendering|Material|CreateDynamicMaterialInstance "/Game/Foliage/Tree01/Tree_Branches_2_Mat.Tree_Branches_2_Mat" :!class /Script/Engine.KismetMaterialLibrary))
  (bind _output_get_3 (Variables|Default|SetTreeMat2 _returnvalue_3))
  (Rendering|Material|SetMaterial Tree 2 _output_get)
  (Rendering|Material|SetMaterial Tree 0 _output_get_2)
  (Rendering|Material|SetMaterial Tree 1 _output_get_3))