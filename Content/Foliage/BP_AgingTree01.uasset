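; Tree actor that ages or rejuvenates when AgeTree or OnTimeGun fires, alternating direction each time and ignoring triggers mid-transition.
; The construction script creates dynamic materials for leaves and two branch slots.
; One timeline, played forward or reversed, drives their age and darkness parameters, then flips the Young state.
; Falling-leaf particles start when aging begins and stop at a timeline event while still Young.
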(event Custom|AgeTree
  (if (not (Variables|Default|GetAging))
    (if (Variables|Default|GetYoung)
      (Variables|Default|SetAging true)
      (Components|Activation|SetActive (Variables|Default|GetFallingLeafs) true false)
      (bind (_direction _age _darkness _branchdarkness) (Timeline|Timeline_0 PlayFromStart)
        (:Update
          (Rendering|Material|SetScalarParameterValue (Variables|Default|GetLeavesMat) "Age" _age :!class /Script/Engine.MaterialInstanceDynamic)
          (Rendering|Material|SetScalarParameterValue (Variables|Default|GetLeavesMat) "BranchDarkness" _branchdarkness :!class /Script/Engine.MaterialInstanceDynamic)
          (Rendering|Material|SetScalarParameterValue (Variables|Default|GetTreeMat1) "Darkness" _darkness :!class /Script/Engine.MaterialInstanceDynamic)
          (Rendering|Material|SetScalarParameterValue (Variables|Default|GetTreeMat2) "Darkness" _darkness :!class /Script/Engine.MaterialInstanceDynamic))
        (:Finished
          (if (Variables|Default|GetYoung)
            (Variables|Default|SetYoung false)
            (else
              (Variables|Default|SetYoung true)))
          (Variables|Default|SetAging false))
        (:ParticleStop
          (if (Variables|Default|GetYoung)
            (Components|Activation|SetActive (Variables|Default|GetFallingLeafs) false false))))
      (else
        (Variables|Default|SetAging true)
        (Timeline|Timeline_0 ReverseFromEnd)))))

(event EventBeginPlay
  (Components|Activation|SetActive (Variables|Default|GetFallingLeafs) false true))

(event Collision|EventActorBeginOverlap
  (params (OtherActor :type Actor%20Object%20Reference)))

(event EventTick
  (params (DeltaSeconds :type Float%20%28single-precision%29)))

(event EventOnTimeGun
  (params (Location :type Vector :default "0, 0, 0"))
  (if (not (Variables|Default|GetAging))
    (if (Variables|Default|GetYoung)
      (Variables|Default|SetAging true)
      (Components|Activation|SetActive (Variables|Default|GetFallingLeafs) true false)
      (bind (_direction _age _darkness _branchdarkness) (Timeline|Timeline_0 PlayFromStart)
        (:Update
          (Rendering|Material|SetScalarParameterValue (Variables|Default|GetLeavesMat) "Age" _age :!class /Script/Engine.MaterialInstanceDynamic)
          (Rendering|Material|SetScalarParameterValue (Variables|Default|GetLeavesMat) "BranchDarkness" _branchdarkness :!class /Script/Engine.MaterialInstanceDynamic)
          (Rendering|Material|SetScalarParameterValue (Variables|Default|GetTreeMat1) "Darkness" _darkness :!class /Script/Engine.MaterialInstanceDynamic)
          (Rendering|Material|SetScalarParameterValue (Variables|Default|GetTreeMat2) "Darkness" _darkness :!class /Script/Engine.MaterialInstanceDynamic))
        (:Finished
          (if (Variables|Default|GetYoung)
            (Variables|Default|SetYoung false)
            (else
              (Variables|Default|SetYoung true)))
          (Variables|Default|SetAging false))
        (:ParticleStop
          (if (Variables|Default|GetYoung)
            (Components|Activation|SetActive (Variables|Default|GetFallingLeafs) false false))))
      (else
        (Variables|Default|SetAging true)
        (Timeline|Timeline_0 ReverseFromEnd)))))

(fn ConstructionScript
  (bind _tree (Variables|Default|GetTree))
  (bind _returnvalue (Rendering|Material|CreateDynamicMaterialInstance "/Game/Foliage/Tree01/Tree_Leaves_Mat_2.Tree_Leaves_Mat_2" :!class /Script/Engine.KismetMaterialLibrary))
  (bind _output_get (Variables|Default|SetLeavesMat _returnvalue))
  (Rendering|Material|SetScalarParameterValue _output_get "Age" 1e+01 :!class /Script/Engine.MaterialInstanceDynamic)
  (bind _returnvalue_2 (Rendering|Material|CreateDynamicMaterialInstance "/Game/Foliage/Tree01/Tree_Branches_Mat.Tree_Branches_Mat" :!class /Script/Engine.KismetMaterialLibrary))
  (bind _output_get_2 (Variables|Default|SetTreeMat1 _returnvalue_2))
  (bind _returnvalue_3 (Rendering|Material|CreateDynamicMaterialInstance "/Game/Foliage/Tree01/Tree_Branches_2_Mat.Tree_Branches_2_Mat" :!class /Script/Engine.KismetMaterialLibrary))
  (bind _output_get_3 (Variables|Default|SetTreeMat2 _returnvalue_3))
  (Rendering|Material|SetMaterial _tree 2 _output_get)
  (Rendering|Material|SetMaterial _tree 0 _output_get_2)
  (Rendering|Material|SetMaterial _tree 1 _output_get_3))