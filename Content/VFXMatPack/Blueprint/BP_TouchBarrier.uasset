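; Barrier effect demo actor that plays a repeating impact animation on its plane through a dynamic M_Impact material instance.
; The construction script creates the instance and sets the impact radius.
; Whenever no animation runs, Tick sends a random ImpactPosition, prints a debug string and restarts a timeline that drives ImpactTime.
; Despite the TouchBarrier name, no touch or overlap triggers the impacts.
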(event EventTick
  (params (DeltaSeconds :type Float%20%28single-precision%29))
  (bind _returnvalue (Math|Random|RandomIntegerinRange 0 100))
  (bind _returnvalue_2 (Math|Random|RandomIntegerinRange 0 100))
  (bind _returnvalue_3 (Math|Random|RandomIntegerinRange 0 100))
  (bind _returnvalue_4 (Math|Conversions|ToFloat(Integer) _returnvalue))
  (bind _returnvalue_5 (Math|Conversions|ToFloat(Integer) _returnvalue_2))
  (bind _returnvalue_6 (Math|Conversions|ToFloat(Integer) _returnvalue_3))
  (bind _linearcolor (Utilities|Struct|MakeLinearColor _returnvalue_5 _returnvalue_6 _returnvalue_4 1.0))
  (if (not (Variables|Default|GetAnimation))
    (Variables|Default|SetAnimation true)
    (Rendering|Material|SetVectorParameterValue (Variables|Default|GetImpactMat) "ImpactPosition" _linearcolor :!class /Script/Engine.MaterialInstanceDynamic)
    (Development|PrintString "Hello" true true _linearcolor)
    (bind _time (Timeline|Timeline_0 PlayFromStart)
      (:Update
        (Rendering|Material|SetScalarParameterValue (Variables|Default|GetImpactMat) "ImpactTime" _time :!class /Script/Engine.MaterialInstanceDynamic))
      (:Finished
        (Variables|Default|SetAnimation false)))))

(event EventBeginPlay)

(event EventActorBeginOverlap
  (params (OtherActor :type Actor%20Object%20Reference)))

(fn ConstructionScript
  (bind _returnvalue (Rendering|Material|CreateDynamicMaterialInstance 0 "/Game/VFXMatPack/Materials/M_Impact.M_Impact" :!class /Script/Engine.PrimitiveComponent))
  (bind _output_get (Variables|Default|SetImpactMat _returnvalue))
  (Rendering|Material|SetMaterial (Variables|Default|GetPlane) 0 _output_get)
  (Rendering|Material|SetScalarParameterValue _output_get "ImpactRadius" 6e+02 :!class /Script/Engine.MaterialInstanceDynamic))