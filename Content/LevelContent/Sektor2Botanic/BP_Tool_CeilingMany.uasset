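; Level-building tool that tiles a rectangular ceiling from instanced static meshes on a 200-unit grid.
; The construction script flattens Size to X and Y, creates an instanced mesh component and adds one instance per grid cell.
; EmptyFields leaves holes by skipping any cell that strictly contains one of the points in the EmptyFields array.
; GetSize returns Size in tile units, and the event graph holds no logic.
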(event EventBeginPlay)

(event Collision|EventActorBeginOverlap
  (params (OtherActor :type Actor%20Object%20Reference)))

(event EventTick
  (params (DeltaSeconds :type Float%20%28single-precision%29)))

(fn ConstructionScript
  (bind _returnvalue (AddComponent|AddInstancedStaticMeshComponent false))
  (Variables|Default|SetFloorElement _returnvalue)
  ;[1 1 1] Only X and Y scaling allowed
  (bind _output_get (Variables|Default|SetSize (Math|Vector|MakeVector (.X (Math|Vector|BreakVector (Variables|Default|GetSize))) (.Y (Math|Vector|BreakVector (Variables|Default|GetSize))) 0.0)))
  ;[1 1 1] For X and Y
  (for _index (range 0 (.ReturnValue (Math|Float|Division(WholeandRemainder) (.X (Math|Vector|BreakVector _output_get)) 2e+02)))
    (for _index_2 (range 0 (.ReturnValue (Math|Float|Division(WholeandRemainder) (.Y (Math|Vector|BreakVector _output_get)) 2e+02)))
      (bind _empty_ (CallFunction|EmptyFields? _index _index_2))
      (if (not _empty_)
        ;[1 1 1] Add Instances
        (Components|InstancedStaticMesh|AddInstance (Variables|Default|GetFloorElement) (Math|Transform|MakeTransform (+ (Math|Vector|MakeVector (* _index 2e+02) (* _index_2 2e+02) 0.0) "200.000000,0.000000, 0")))))))

(fn GetSize
  (bind _size (Variables|Default|GetSize))
  (bind _returnvalue (/ _size 2e+02))
  (return (Math|Vector|MakeVector (.x _returnvalue) (.y _returnvalue) 1.0)))

(fn EmptyFields?
  (params (IndexX :type Integer) (IndexY :type Integer))
  (bind _returnvalue (* IndexY 2e+02))
  (bind _returnvalue_2 (* IndexX 2e+02))
  (bind _array_element (Utilities|Array|ForEachLoopwithBreak (Variables|Default|GetEmptyFields))
    (:LoopBody
      (if (and (and (< (* (.X (Math|Vector|BreakVector _array_element)) 1.0) (+ _returnvalue_2 2e+02)) (> (* (.X (Math|Vector|BreakVector _array_element)) 1.0) _returnvalue_2)) (and (< (* (.Y (Math|Vector|BreakVector _array_element)) 1.0) (+ _returnvalue 2e+02)) (> (* (.Y (Math|Vector|BreakVector _array_element)) 1.0) _returnvalue)))
        (Variables|Default|SetTemp true)
        (return (Variables|Default|GetTemp))))
    (:Completed
      (Variables|Default|SetTemp false)
      (return (Variables|Default|GetTemp)))))