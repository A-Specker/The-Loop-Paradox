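; BP_FloorRoom is a procedural floor builder for a room in the Sektor2Botanic level content, tiling a mesh over a configurable area.
; Its construction script creates an instanced static mesh component, applies the chosen material and makes Size positive and flat.
; Nested loops over Size divided by ElementSize place instances on an XY grid, scaled uniformly relative to a 200-unit base.
; It has no active runtime logic.
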(event EventBeginPlay)

(event Collision|EventActorBeginOverlap
  (params (OtherActor :type Actor%20Object%20Reference)))

(event EventTick
  (params (DeltaSeconds :type Float%20%28single-precision%29)))

(fn ConstructionScript
  (bind _elementsize (Variables|Default|GetElementSize))
  (bind _elementsize_2 (Variables|Default|GetElementSize))
  (bind _elementsize_3 (Variables|Default|GetElementSize))
  (bind _returnvalue (/ _elementsize_2 2e+02))
  (bind _returnvalue_2 (AddComponent|AddInstancedStaticMeshComponent false))
  (bind _output_get (Variables|Default|SetFloorElem _returnvalue_2))
  (Rendering|Material|SetMaterial _output_get 0 (Variables|Default|GetMaterial))
  (bind _output_get_2 (Variables|Default|SetSize (Math|Vector|MakeVector (Math|Float|Absolute(Float) (.X (Math|Vector|BreakVector (Variables|Default|GetSize)))) (Math|Float|Absolute(Float) (.Y (Math|Vector|BreakVector (Variables|Default|GetSize)))) 0.0)))
  (for _index (range 0 (.ReturnValue (Math|Float|Division(WholeandRemainder) (.X (Math|Vector|BreakVector _output_get_2)) _elementsize_3)))
    (for _index_2 (range 0 (.ReturnValue (Math|Float|Division(WholeandRemainder) (.Y (Math|Vector|BreakVector _output_get_2)) _elementsize_3)))
      (Components|InstancedStaticMesh|AddInstance (Variables|Default|GetFloorElem) (Math|Transform|MakeTransform (Math|Vector|MakeVector (* _index _elementsize) (* _index_2 _elementsize) 0.0) "0, 0, 0" (Math|Vector|MakeVector _returnvalue _returnvalue _returnvalue))))))