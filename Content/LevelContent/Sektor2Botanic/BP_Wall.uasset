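; BP_Wall is a construction-script wall builder in the Sektor2Botanic level content that lays out repeated segments along local X.
; It forces Size to a non-negative X with zero Y and Z, then derives the segment count from how many whole 400-unit steps fit.
; An instanced static mesh component created at construction holds the evenly spaced, unrotated instances.
; The event graph has no active logic.
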(event EventBeginPlay)

(event Collision|EventActorBeginOverlap
  (params (OtherActor :type Actor%20Object%20Reference)))

(event EventTick
  (params (DeltaSeconds :type Float%20%28single-precision%29)))

(fn ConstructionScript
  (bind _returnvalue (AddComponent|AddInstancedStaticMeshComponent false))
  (Variables|Default|SetWallElem _returnvalue)
  (bind _output_get (Variables|Default|SetSize (Math|Vector|MakeVector (Math|Float|Absolute(Float) (.X (Math|Vector|BreakVector (Variables|Default|GetSize)))) 0.0 0.0)))
  (for _index (range 1 (.ReturnValue (Math|Float|Division(WholeandRemainder) (.X (Math|Vector|BreakVector _output_get)) 4e+02)))
    (Components|InstancedStaticMesh|AddInstance (Variables|Default|GetWallElem) (Math|Transform|MakeTransform (Math|Vector|MakeVector (* _index 4e+02) 0.0 0.0) "0, 0, 0" "1.000000,1.000000,1.000000"))))