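; BP_StreamChamber is a two-door transition chamber in the Botanic sector that swaps streamed levels as something passes through.
; Start and end triggers set the current side and re-arm the chamber.
; The central trigger toggles that side's door, waits, calls level streaming to unload one level and load the other, then toggles the opposite door.
; Level enums resolve to names through a construction-built string list, and BeginPlay toggles any open door after a delay.
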(event OnComponentBeginOverlap(Box)
  (params (OtherActor :type Actor%20Object%20Reference) (OtherComp :type Primitive%20Component%20Object%20Reference) (OtherBodyIndex :type Integer) (bFromSweep :type Boolean) (SweepResult :type Hit%20Result%20Structure%20%28by%20ref%29))
  (if (Variables|Default|GetUsable)
    (Variables|Default|SetUsable false)
    (switch int (Variables|Default|GetLevel)
      (:0
        (Variables|Default|SetLevel 1)
        (Class|InteractInterface|OnInteract(Message) (.AsBP%20Door%20Open%20Botanic (Utilities|Casting|CastToBP_DoorOpenBotanic (Variables|/Script/Engine.ChildActorComponent|GetChildActor (Variables|Default|GetBP_DoorOpenBotanic)))))
        (Utilities|FlowControl|Delay 2.0)
        (bind _returnvalue (CallFunction|LevelnametoNameFunction (Variables|Default|GetLevelStart)))
        (bind _returnvalue_2 (CallFunction|LevelnametoNameFunction (Variables|Default|GetLevelEnd)))
        (Development|PrintString _returnvalue_2)
        (Default|CallLevelStream _returnvalue _returnvalue_2)
        (Class|InteractInterface|OnInteract(Message) (.AsBP%20Door%20Open%20Botanic (Utilities|Casting|CastToBP_DoorOpenBotanic (Variables|/Script/Engine.ChildActorComponent|GetChildActor (Variables|Default|GetBP_DoorOpenBotanic1))))))
      (:1
        (Variables|Default|SetLevel 0)
        (Class|InteractInterface|OnInteract(Message) (.AsBP%20Door%20Open%20Botanic (Utilities|Casting|CastToBP_DoorOpenBotanic (Variables|/Script/Engine.ChildActorComponent|GetChildActor (Variables|Default|GetBP_DoorOpenBotanic1)))))
        (Utilities|FlowControl|Delay 2.0)
        (bind _returnvalue_3 (CallFunction|LevelnametoNameFunction (Variables|Default|GetLevelStart)))
        (bind _returnvalue_4 (CallFunction|LevelnametoNameFunction (Variables|Default|GetLevelEnd)))
        (Default|CallLevelStream _returnvalue_4 _returnvalue_3)
        (Class|InteractInterface|OnInteract(Message) (.AsBP%20Door%20Open%20Botanic (Utilities|Casting|CastToBP_DoorOpenBotanic (Variables|/Script/Engine.ChildActorComponent|GetChildActor (Variables|Default|GetBP_DoorOpenBotanic)))))))))

(event OnComponentBeginOverlap(BoxStart)
  (params (OtherActor :type Actor%20Object%20Reference) (OtherComp :type Primitive%20Component%20Object%20Reference) (OtherBodyIndex :type Integer) (bFromSweep :type Boolean) (SweepResult :type Hit%20Result%20Structure%20%28by%20ref%29))
  (Variables|Default|SetLevel 0)
  (Variables|Default|SetUsable true))

(event OnComponentBeginOverlap(BoxEnd)
  (params (OtherActor :type Actor%20Object%20Reference) (OtherComp :type Primitive%20Component%20Object%20Reference) (OtherBodyIndex :type Integer) (bFromSweep :type Boolean) (SweepResult :type Hit%20Result%20Structure%20%28by%20ref%29))
  (Variables|Default|SetLevel 1)
  (Variables|Default|SetUsable true))

(event EventBeginPlay
  (bind _bp_dooropenbotanic (Variables|Default|GetBP_DoorOpenBotanic))
  (bind _bp_dooropenbotanic1 (Variables|Default|GetBP_DoorOpenBotanic1))
  (bind _childactor (Variables|/Script/Engine.ChildActorComponent|GetChildActor _bp_dooropenbotanic))
  (bind _childactor_2 (Variables|/Script/Engine.ChildActorComponent|GetChildActor _bp_dooropenbotanic1))
  (bind _asbp_door_open_botanic (Utilities|Casting|CastToBP_DoorOpenBotanic _childactor_2))
  (bind _asbp_door_open_botanic_2 (Utilities|Casting|CastToBP_DoorOpenBotanic _childactor))
  (Utilities|FlowControl|Delay 3.0)
  (if (Variables|/Game/LevelContent/Sektor2Botanic/BP_DoorOpenBotanic.BP_DoorOpenBotanic_C|GetOpen? _asbp_door_open_botanic_2)
    (Development|PrintString "1T")
    (Class|InteractInterface|OnInteract(Message) _asbp_door_open_botanic_2))
  (if (Variables|/Game/LevelContent/Sektor2Botanic/BP_DoorOpenBotanic.BP_DoorOpenBotanic_C|GetOpen? _asbp_door_open_botanic)
    (Development|PrintString "2T")
    (Class|InteractInterface|OnInteract(Message) _asbp_door_open_botanic)))

(fn ConstructionScript
  (bind _enumvalue (|ForEachLevels)
    (:LoopBody
      (Utilities|Array|AppendArray (Variables|Default|GetLevelString) (Utilities|Array|MakeArray (Utilities|String|EnumtoString _enumvalue))))))

(fn LevelnametoNameFunction
  (params (Input :type Levels%20Enum))
  (bind _returnvalue (Utilities|String|EnumtoString Input))
  (bind _array_element (Utilities|Array|ForEachLoopwithBreak (Variables|Default|GetLevelString) :!label _label)
    (:LoopBody
      (if (Utilities|Enum|Equal(Enum) _array_element _returnvalue)
        (bind _output_get (Variables|Default|SetNameTest (Utilities|String|StringToName _returnvalue)))
        (goto _label Break)))
    (:Completed
      (return (Utilities|String|ToString(Name) _output_get)))))