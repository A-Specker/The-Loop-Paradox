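; BP_Shield is a shield plane in the Botanic sector that reacts to time gun hits and is removed once the laser puzzle is solved.
; Construction gives the plane a dynamic material; OnTimeGun sets an offset, actor-relative impact position on it, and a timeline animates ImpactTime.
; Off moves the plane far upward instead of destroying it, and BeginPlay calls it when the loaded save has LaserSolved set.
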(event Custom|Off
  (Transformation|AddLocalOffset (Variables|Default|GetPlane) "0, 0,200000.000000" false))

(event Collision|EventActorBeginOverlap
  (params (OtherActor :type Actor%20Object%20Reference)))

(event EventTick
  (params (DeltaSeconds :type Float%20%28single-precision%29)))

(event EventOnTimeGun
  (params (Location :type Vector))
  (bind _returnvalue (Transformation|GetActorLocation))
  (bind _returnvalue_2 (- Location _returnvalue))
  (bind (_x _y _z) (Math|Vector|BreakVector _returnvalue_2))
  (Rendering|Material|SetVectorParameterValue (Variables|Default|GetMaterial) "ImpactPosition" (Math|Conversions|ToLinearColor(Vector) (Math|Vector|MakeVector 0.0 (- _y 425.0) (- _z 425.0))) :!class /Script/Engine.MaterialInstanceDynamic)
  (bind _newtrack_0 (Timeline|Timeline_0 PlayFromStart)
    (:Update
      (Rendering|Material|SetScalarParameterValue (Variables|Default|GetMaterial) "ImpactTime" _newtrack_0 :!class /Script/Engine.MaterialInstanceDynamic))))

(event EventBeginPlay
  (bind _returnvalue (SaveGame|LoadGamefromSlot "GameSaveSlot"))
  (bind _output_get (Variables|Default|SetGameSave _returnvalue))
  (if (Variables|/Game/SaveGame/GameSaver.GameSaver_C|GetLaserSolved (.AsGame%20Saver (Utilities|Casting|CastToGameSaver _output_get)))
    (CallFunction|Off)))

(fn ConstructionScript
  (bind _returnvalue (Rendering|Material|CreateDynamicMaterialInstance "/Game/VFXMatPack/MaterialInstance/MI_Shield.MI_Shield" :!class /Script/Engine.KismetMaterialLibrary))
  (bind _output_get (Variables|Default|SetMaterial _returnvalue))
  (Rendering|Material|SetMaterial (Variables|Default|GetPlane) 0 _output_get))