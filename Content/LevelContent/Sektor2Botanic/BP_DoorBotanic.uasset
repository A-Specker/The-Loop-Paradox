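; Sliding door for the Sektor2 Botanic level that moves its inner panel vertically, with an optional malfunction mode.
; TriggerDoor plays or reverses the Position timeline with open and close sounds, ignoring calls while moving.
; When Error is set, a timeline started at BeginPlay drives the panel and triggers bang sounds until Shut.
; ShutDoor runs once, silencing the malfunction and playing a closing timeline that ends with a bang.
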(event Custom|TriggerDoor
  (if (not (Variables|Default|GetIsMoving))
    (Variables|Default|SetIsMoving true)
    (if (Variables|Default|GetIsDown)
      (Class|GameplayStatics|PlaySoundAttached "/Game/Audio/Sounds/DoorSlideClose_Cue.DoorSlideClose_Cue" (Variables|Default|Getdoor))
      (bind _position (Timeline|Position ReverseFromEnd)
        (:Update
          (Transformation|SetRelativeLocation (Variables|Default|Getdoor_inner) (Math|Vector|MakeVector 0.0 0.0 _position) false))
        (:Finished
          (Variables|Default|SetIsMoving false)
          (if (Variables|Default|GetIsDown)
            (Variables|Default|SetIsDown false)
            (else
              (Variables|Default|SetIsDown true)))))
      (else
        (Class|GameplayStatics|PlaySoundAttached "/Game/Audio/Sounds/DoorSlideOpen_Cue.DoorSlideOpen_Cue" (Variables|Default|Getdoor))
        (Timeline|Position Play)))))

(event Custom|Shut%20Door
  ;[1 1 1] Close Door for Good
  (if (not (Variables|Default|GetShut?))
    (Variables|Default|SetShut? true)
    (bind _shutthedoor (Timeline|Kek Play)
      (:Update
        (Transformation|SetRelativeLocation (Variables|Default|Getdoor_inner) (Math|Vector|MakeVector 0.0 0.0 _shutthedoor) false))
      (:Finished
        (Class|GameplayStatics|PlaySoundAttached "/Game/Audio/Sounds/DoorCloseBang_Cue.DoorCloseBang_Cue" (Variables|Default|Getdoor))))))

(event EventBeginPlay
  ;[1 1 1] Error
  (if (Variables|Default|GetError?)
    (bind _position (Timeline|Error Play)
      (:Update
        (if (not (Variables|Default|GetShut?))
          (Transformation|SetRelativeLocation (Variables|Default|Getdoor_inner) (Math|Vector|MakeVector 0.0 0.0 _position) false)))
      (:Play%20Sound
        (if (not (Variables|Default|GetShut?))
          (Class|GameplayStatics|PlaySoundAttached "/Game/Audio/Sounds/DoorBang.DoorBang" (Variables|Default|Getdoor)))))))

(fn ConstructionScript)