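; Interactable door terminal for the Botanic sector that opens and closes its child-actor door.
; Interacting while locked flashes red with an error sound; otherwise it turns green, plays a success sound, triggers the door and saves Open, with a timeline resetting the color.
; GameSaver stores door states keyed by actor location, restored on BeginPlay.
; The construction script pre-positions open doors but casts to BP_Door rather than BP_DoorBotanic.
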(event EventBeginPlay
  (bind _returnvalue (Transformation|GetActorLocation))
  (bind _returnvalue_2 (SaveGame|DoesSaveGameExist (Variables|Default|GetGameSave)))
  (if _returnvalue_2
    (bind _returnvalue_3 (SaveGame|LoadGamefromSlot (Variables|Default|GetGameSave)))
    (bind _output_get (Variables|Default|SetSaveGameRef _returnvalue_3))
    (bind _asgame_saver (Utilities|Casting|CastToGameSaver _output_get))
    (if (== (Utilities|Array|FindItem (Variables|/Game/SaveGame/GameSaver.GameSaver_C|GetDoors _asgame_saver) _returnvalue) -1)
      (bind _returnvalue_4 (Utilities|Array|Add (Variables|/Game/SaveGame/GameSaver.GameSaver_C|GetDoors (.AsGame%20Saver (Utilities|Casting|CastToGameSaver (Variables|Default|GetSaveGameRef)))) _returnvalue))
      (Utilities|Array|SetArrayElem (Variables|/Game/SaveGame/GameSaver.GameSaver_C|GetDoorOpen (.AsGame%20Saver (Utilities|Casting|CastToGameSaver (Variables|Default|GetSaveGameRef)))) _returnvalue_4 (Variables|Default|GetOpen?) true)
      (SaveGame|SaveGametoSlot (Variables|Default|GetSaveGameRef) (Variables|Default|GetGameSave))
      (elif (not (Math|Boolean|Equal(Boolean) (Variables|Default|GetOpen?) (Utilities|Array|Get(acopy) (Variables|/Game/SaveGame/GameSaver.GameSaver_C|GetDoorOpen (.AsGame%20Saver (Utilities|Casting|CastToGameSaver (Variables|Default|GetSaveGameRef)))) (Utilities|Array|FindItem (Variables|/Game/SaveGame/GameSaver.GameSaver_C|GetDoors _asgame_saver) _returnvalue))))
        (Variables|Default|SetOpen? (Utilities|Array|Get(acopy) (Variables|/Game/SaveGame/GameSaver.GameSaver_C|GetDoorOpen (.AsGame%20Saver (Utilities|Casting|CastToGameSaver (Variables|Default|GetSaveGameRef)))) (Utilities|Array|FindItem (Variables|/Game/SaveGame/GameSaver.GameSaver_C|GetDoors _asgame_saver) _returnvalue)))
        (Default|TriggerDoor (.AsBP%20Door%20Botanic (Utilities|Casting|CastToBP_DoorBotanic (Variables|/Script/Engine.ChildActorComponent|GetChildActor (Variables|Default|GetBP_TestDoor)))))))))

(event EventOnInteract
  (bind _sm_doorterminal (Variables|Default|GetSM_DoorTerminal))
  (if (Variables|Default|GetLocked?)
    (Rendering|Material|SetVectorParameterValue (Variables|Default|GetMaterial) "Color" "(R=0.600000,G=0.079729,B=0.075000,A=1.000000)" :!class /Script/Engine.MaterialInstanceDynamic)
    (Class|GameplayStatics|PlaySoundAttached "/Game/Audio/Sounds/SpaceshipInterfaceError_Cue.SpaceshipInterfaceError_Cue" _sm_doorterminal)
    (Timeline|Timer PlayFromStart
      (:Finished
        (Rendering|Material|SetVectorParameterValue (Variables|Default|GetMaterial) "Color" "(R=0.376471,G=0.490196,B=1.000000,A=0.000000)" :!class /Script/Engine.MaterialInstanceDynamic)))
    (else
      (Rendering|Material|SetVectorParameterValue (Variables|Default|GetMaterial) "Color" "(R=0.079781,G=0.620000,B=0.096582,A=1.000000)" :!class /Script/Engine.MaterialInstanceDynamic)
      (Class|GameplayStatics|PlaySoundAttached "/Game/Audio/Sounds/SpaceshipInterfaceSuccess_Cue.SpaceshipInterfaceSuccess_Cue" _sm_doorterminal)
      (Default|TriggerDoor (.AsBP%20Door%20Botanic (Utilities|Casting|CastToBP_DoorBotanic (Variables|/Script/Engine.ChildActorComponent|GetChildActor (Variables|Default|GetBP_TestDoor)))))
      (if (Variables|Default|GetOpen?)
        (Variables|Default|SetOpen? false)
        (else
          (Variables|Default|SetOpen? true)))
      (CallFunction|SaveDoor)
      (Timeline|Timer PlayFromStart))))

(fn ConstructionScript
  (bind _returnvalue (Rendering|Material|CreateDynamicMaterialInstance "/Game/General/Sources/DoorTerminal/M_DoorTerminal.M_DoorTerminal" :!class /Script/Engine.KismetMaterialLibrary))
  (bind _output_get (Variables|Default|SetMaterial _returnvalue))
  (Rendering|Material|SetMaterial (Variables|Default|GetSM_DoorTerminal) 0 _output_get)
  (if (Variables|Default|GetOpen?)
    (bind _asbp_door (Utilities|Casting|CastToBP_Door (Variables|/Script/Engine.ChildActorComponent|GetChildActor (Variables|Default|GetBP_TestDoor))))
    (Transformation|SetRelativeLocation (Variables|/Game/Blueprints/BP_Door.BP_Door_C|Getdoor_inner _asbp_door) (Math|Vector|MakeVector (.X (Math|Vector|BreakVector (Variables|/Script/Engine.SceneComponent|GetRelativeLocation (Variables|/Game/Blueprints/BP_Door.BP_Door_C|Getdoor_inner _asbp_door)))) (.Y (Math|Vector|BreakVector (Variables|/Script/Engine.SceneComponent|GetRelativeLocation (Variables|/Game/Blueprints/BP_Door.BP_Door_C|Getdoor_inner _asbp_door)))) -399.0) false)))

(fn SaveDoor
  (bind _returnvalue (SaveGame|LoadGamefromSlot (Variables|Default|GetGameSave)))
  (bind _output_get (Variables|Default|SetSaveGameRef _returnvalue))
  (bind _asgame_saver (Utilities|Casting|CastToGameSaver _output_get))
  (Utilities|Array|SetArrayElem (Variables|/Game/SaveGame/GameSaver.GameSaver_C|GetDoorOpen _asgame_saver) (Utilities|Array|FindItem (Variables|/Game/SaveGame/GameSaver.GameSaver_C|GetDoors _asgame_saver) (Transformation|GetActorLocation)) (Variables|Default|GetOpen?))
  (SaveGame|SaveGametoSlot (Variables|Default|GetSaveGameRef) (Variables|Default|GetGameSave)))