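; Laboratory wall element that builds a resizable wall from tiled instances of one static mesh in the Construction Script.
; Size snaps to whole 100-unit Y and 300-unit Z steps, with X fixed at -100.
; Nested loops fill the Y/Z grid on an instanced mesh component created on the first column.
; Each column also adds a base instance, duplicating the bottom cell when Z loops run.
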(event EventBeginPlay)

(event Collision|EventActorBeginOverlap
  (params (OtherActor :type Actor%20Object%20Reference)))

(event EventTick
  (params (DeltaSeconds :type Float%20%28single-precision%29)))

(fn ConstructionScript
  ;[1 1 1] Stabilize Vector
  (bind _output_get (Variables|Default|SetSize (Math|Vector|MakeVector -1e+02 (CallFunction|ClampVectorY (.Y (Math|Vector|BreakVector (Variables|Default|GetSize)))) (CallFunction|ClampVectorZ (.Z (Math|Vector|BreakVector (Variables|Default|GetSize)))))))
  ;[1 1 1] Y - Shelves
  (for _index (range 0 (- (.ReturnValue (Math|Float|Division(WholeandRemainder) (.Y (Math|Vector|BreakVector _output_get)) 1e+02)) 1))
    ;;[1 1 1] Add Static Mesh
    (if (== _index 0)
      (bind _returnvalue (AddComponent|AddInstancedStaticMeshComponent false))
      (Variables|Default|SetInstancedStaticMesh _returnvalue))
    (Components|InstancedStaticMesh|AddInstance (Variables|Default|GetInstancedStaticMesh) (Math|Transform|MakeTransform (Math|Vector|MakeVector 0.0 (* _index 1e+02) 0.0)))
    ;[1 1 1] Z
    ;  - Shelves
    (for _index_2 (range 0 (- (.ReturnValue (Math|Float|Division(WholeandRemainder) (.Z (Math|Vector|BreakVector (Variables|Default|GetSize))) 3e+02)) 1))
      (Components|InstancedStaticMesh|AddInstance (Variables|Default|GetInstancedStaticMesh) (Math|Transform|MakeTransform (Math|Vector|MakeVector 0.0 (* _index 1e+02) (* _index_2 3e+02)))))))

(fn ClampVectorY
  (params (Input :type Float%20%28single-precision%29 :default 0.0))
  (return (- Input (.Remainder (Math|Float|Division(WholeandRemainder) Input 1e+02)))))

(fn ClampVectorZ
  (params (Input :type Float%20%28single-precision%29 :default 0.0))
  (return (- Input (.Remainder (Math|Float|Division(WholeandRemainder) Input 3e+02)))))