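; Laboratory specimen tube prop with configurable emissive base, top and lamp sections plus a matching spotlight.
; The construction script creates a dynamic material instance and applies each section's strength and color, scaling spotlight intensity from lamp strength.
; When LightsOff is set, BeginPlay dims the emissives and spotlight to OffValue.
; The HorrorLightsOn event restores the configured glow and light.
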(event Custom|HorrorLightsOn
  ;[1 1 1] Base
  (Rendering|Material|SetScalarParameterValue (Variables|Default|GetMaterial) "Emmisive Base" (Variables|Default|GetBaseStrength) :!class /Script/Engine.MaterialInstanceDynamic)
  (Rendering|Material|SetVectorParameterValue (Variables|Default|GetMaterial) "BaseColor" (Variables|Default|GetBaseColor) :!class /Script/Engine.MaterialInstanceDynamic)
  ;[1 1 1] Top
  (Rendering|Material|SetScalarParameterValue (Variables|Default|GetMaterial) "Emmisive Top" (Variables|Default|GetTopStrength) :!class /Script/Engine.MaterialInstanceDynamic)
  (Rendering|Material|SetVectorParameterValue (Variables|Default|GetMaterial) "TopColor" (Variables|Default|GetTopColor) :!class /Script/Engine.MaterialInstanceDynamic)
  ;[1 1 1] Lamp
  (Rendering|Material|SetScalarParameterValue (Variables|Default|GetMaterial) "Emmisive Lamp" (Variables|Default|GetLampStrength) :!class /Script/Engine.MaterialInstanceDynamic)
  (Rendering|Material|SetVectorParameterValue (Variables|Default|GetMaterial) "LampColor" (Variables|Default|GetLampColor) :!class /Script/Engine.MaterialInstanceDynamic)
  (Rendering|Components|Light|SetIntensity (Variables|Default|GetSpotLight) (* (Variables|Default|GetLampStrength) (Variables|Default|GetLampLightMult)))
  (Rendering|Components|Light|SetLightColor (Variables|Default|GetSpotLight) (Variables|Default|GetLampColor))
  (Rendering|Material|SetMaterial 0 (Variables|Default|GetMaterial)))

(event EventBeginPlay
  (if (Variables|Default|GetLightsOff)
    ;[1 1 1] Base
    (Rendering|Material|SetScalarParameterValue (Variables|Default|GetMaterial) "Emmisive Base" (Variables|Default|GetOffValue) :!class /Script/Engine.MaterialInstanceDynamic)
    ;[1 1 1] Top
    (Rendering|Material|SetScalarParameterValue (Variables|Default|GetMaterial) "Emmisive Top" (Variables|Default|GetOffValue) :!class /Script/Engine.MaterialInstanceDynamic)
    ;[1 1 1] Lamp
    (Rendering|Material|SetScalarParameterValue (Variables|Default|GetMaterial) "Emmisive Lamp" (Variables|Default|GetOffValue) :!class /Script/Engine.MaterialInstanceDynamic)
    (Rendering|Components|Light|SetIntensity (Variables|Default|GetSpotLight) (Variables|Default|GetOffValue))
    (Rendering|Material|SetMaterial 0 (Variables|Default|GetMaterial))))

(event Collision|EventActorBeginOverlap
  (params (OtherActor :type Actor%20Object%20Reference)))

(event EventTick
  (params (DeltaSeconds :type Float%20%28single-precision%29)))

(fn ConstructionScript
  (bind _returnvalue (Rendering|Material|CreateDynamicMaterialInstance 0 0 :!class /Script/Engine.PrimitiveComponent))
  (Variables|Default|SetMaterial _returnvalue)
  ;[1 1 1] Base
  (Rendering|Material|SetScalarParameterValue _returnvalue "Emmisive Base" (Variables|Default|GetBaseStrength) :!class /Script/Engine.MaterialInstanceDynamic)
  (Rendering|Material|SetVectorParameterValue _returnvalue "BaseColor" (Variables|Default|GetBaseColor) :!class /Script/Engine.MaterialInstanceDynamic)
  ;[1 1 1] Top
  (Rendering|Material|SetScalarParameterValue _returnvalue "Emmisive Top" (Variables|Default|GetTopStrength) :!class /Script/Engine.MaterialInstanceDynamic)
  (Rendering|Material|SetVectorParameterValue _returnvalue "TopColor" (Variables|Default|GetTopColor) :!class /Script/Engine.MaterialInstanceDynamic)
  ;[1 1 1] Lamp
  (Rendering|Material|SetScalarParameterValue _returnvalue "Emmisive Lamp" (Variables|Default|GetLampStrength) :!class /Script/Engine.MaterialInstanceDynamic)
  (Rendering|Material|SetVectorParameterValue _returnvalue "LampColor" (Variables|Default|GetLampColor) :!class /Script/Engine.MaterialInstanceDynamic)
  (Rendering|Components|Light|SetIntensity (Variables|Default|GetSpotLight) (* (Variables|Default|GetLampStrength) (Variables|Default|GetLampLightMult)))
  (Rendering|Components|Light|SetLightColor (Variables|Default|GetSpotLight) (Variables|Default|GetLampColor))
  (Rendering|Material|SetMaterial 0 _returnvalue))