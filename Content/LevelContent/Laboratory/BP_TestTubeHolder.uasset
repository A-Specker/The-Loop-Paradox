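; A laboratory test tube holder prop that fills six preset slots with a random arrangement of tubes and plugs.
; The Construction Script adds instanced static mesh components for tubes and plugs, then calls Randomize.
; Each slot randomly receives a tube with random yaw, and only filled slots can get a plug, raised by PlugOffset.
; The event graph is empty.
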(event EventBeginPlay)

(event Collision|EventActorBeginOverlap
  (params (OtherActor :type Actor%20Object%20Reference)))

(event EventTick
  (params (DeltaSeconds :type Float%20%28single-precision%29)))

(fn ConstructionScript
  ;[1 1 1] Add Meshes
  (bind _returnvalue (AddComponent|AddInstancedStaticMeshComponent false))
  (Variables|Default|SetPlug _returnvalue)
  (bind _returnvalue_2 (AddComponent|AddInstancedStaticMeshComponent false))
  (Variables|Default|SetTube _returnvalue_2)
  ;[1 1 1] Randomize?
  (if (Variables|Default|GetRandomize?)
    _
    (else
      _))
  (CallFunction|Randomize)
  (Variables|Default|SetRandomize? false))

(fn Randomize
  ;[1 1 1] Tube 1
  (if (Math|Random|RandomBool)
    (CallFunction|AddTube (Variables|Default|GetLocation01))
    ;[1 1 1] Plug 1
    (if (Math|Random|RandomBool)
      (CallFunction|AddPlug (Variables|Default|GetLocation01))))
  ;[1 1 1] Tube 2
  (if (Math|Random|RandomBool)
    (CallFunction|AddTube (Variables|Default|GetLocation02))
    ;[1 1 1] Plug 2
    (if (Math|Random|RandomBool)
      (CallFunction|AddPlug (Variables|Default|GetLocation02))))
  ;[1 1 1] Tube 3
  (if (Math|Random|RandomBool)
    (CallFunction|AddTube (Variables|Default|GetLocation03))
    ;[1 1 1] Plug 3
    (if (Math|Random|RandomBool)
      (CallFunction|AddPlug (Variables|Default|GetLocation03))))
  ;[1 1 1] Tube 4
  (if (Math|Random|RandomBool)
    (CallFunction|AddTube (Variables|Default|GetLocation04))
    ;[1 1 1] Plug 4
    (if (Math|Random|RandomBool)
      (CallFunction|AddPlug (Variables|Default|GetLocation04))))
  ;[1 1 1] Tube 5
  (if (Math|Random|RandomBool)
    (CallFunction|AddTube (Variables|Default|GetLocation05))
    ;[1 1 1] Plug 5
    (if (Math|Random|RandomBool)
      (CallFunction|AddPlug (Variables|Default|GetLocation05))))
  ;[1 1 1] Tube 5
  (if (Math|Random|RandomBool)
    (CallFunction|AddTube (Variables|Default|GetLocation06))
    ;[1 1 1] Plug 5
    (if (Math|Random|RandomBool)
      (CallFunction|AddPlug (Variables|Default|GetLocation06)))))

(fn GetPlugTransform
  (params (InTransform :type Transform%20%28by%20ref%29))
  (bind (_location _rotation _scale) (Math|Transform|BreakTransform InTransform))
  (bind (_x _y _z) (Math|Vector|BreakVector _location))
  (return (Math|Transform|MakeTransform (Math|Vector|MakeVector _x _y (+ _z (Variables|Default|GetPlugOffset))) _rotation _scale)))

(fn RandomRotation
  (params (InTransform :type Transform%20%28by%20ref%29))
  (bind (_location _rotation) (Math|Transform|BreakTransform InTransform))
  (bind (_pitch _yaw _roll) (Class|KismetMathLibrary|BreakRot _rotation))
  (return (Math|Transform|MakeTransform _location (Class|KismetMathLibrary|MakeRot _pitch (Math|Random|RandomFloatinRange 0.0 3.6e+02) _roll))))

(fn AddTube
  (params (InTransform :type Transform%20%28by%20ref%29))
  (bind _random (CallFunction|RandomRotation InTransform))
  (Components|InstancedStaticMesh|AddInstance (Variables|Default|GetTube) _random)
  (return))

(fn AddPlug
  (params (InTransform :type Transform%20%28by%20ref%29))
  (bind _plugtransform (CallFunction|GetPlugTransform InTransform))
  (Components|InstancedStaticMesh|AddInstance (Variables|Default|GetPlug) _plugtransform))