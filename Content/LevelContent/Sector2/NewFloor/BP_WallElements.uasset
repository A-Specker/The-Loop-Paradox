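; BP_WallElements is a construction-script actor that builds a wall from repeated instanced static meshes.
; The script adds an instanced mesh component, then clamps the Size vector to positive X and Z with zero Y.
; Nested loops over Size divided by the element spacing place unrotated, unscaled instances in a grid on the local XZ plane.
; The event graph holds only disabled placeholder events, so it adds no runtime logic.
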(event EventBeginPlay)

(event Collision|EventActorBeginOverlap
  (params (OtherActor :type Actor%20Object%20Reference)))

(event EventTick
  (params (DeltaSeconds :type Float%20%28single-precision%29)))

(fn ConstructionScript
  (bind _returnvalue (AddComponent|AddInstancedStaticMeshComponent false))
  (Variables|Default|SetWallElement _returnvalue)
  (bind _output_get (Variables|Default|SetSize (Math|Vector|MakeVector (Math|Float|Absolute(Float) (.X (Math|Vector|BreakVector (Variables|Default|GetSize)))) 0.0 (Math|Float|Absolute(Float) (.Z (Math|Vector|BreakVector (Variables|Default|GetSize)))))))
  (for _index (range 0 (.ReturnValue (Math|Float|Division(WholeandRemainder) (.X (Math|Vector|BreakVector _output_get)) 2e+02)))
    (for _index_2 (range 0 (.ReturnValue (Math|Float|Division(WholeandRemainder) (.Z (Math|Vector|BreakVector _output_get)) 1e+02)))
      (Components|InstancedStaticMesh|AddInstance (Variables|Default|GetWallElement) (Math|Transform|MakeTransform (Math|Vector|MakeVector (* _index 2e+02) 0.0 (* _index_2 1e+02)))))))